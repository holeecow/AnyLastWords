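; BP_Weapon is a pickup weapon that the player can equip in the top-down game.
; Sphere overlap sets a flag and binds the weapon to the player controller's pickup-pressed event; leaving clears the flag.
; On press while overlapping, ItemMesh snaps to the character's RightHandSocket and the character state becomes one-handed equipped.
; Tick applies a sine-driven vertical offset, with no check for being equipped.
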(event `OnInteractWithWeapon`
  ; 2. This event triggers when Pickup is pressed
  (if (`self.bOverlapWithPlayer`)
    (bind _asbp_top_down_character (cast `/Game/Characters/Player/Blueprints/BP_TopDownCharacter` (stale `self.Sphere.OnComponentBeginOverlap` OtherActor)))
    ; 3. Attach weapon to the RightHandSocket of the player mesh
    (`SceneComponent.K2_AttachToComponent` (`self.ItemMesh`) (`Character.Mesh` _asbp_top_down_character) "RightHandSocket" "SnapToTarget" "SnapToTarget" "SnapToTarget" true)
    ; 4. Set character state of Player
    (`AnyLastWordsCharacter.SetCharacterState` _asbp_top_down_character "ECS_EquippedOneHandedWeapon")))

(event `self.Sphere.OnComponentBeginOverlap`
  (params (OverlappedComponent :type "PrimitiveComponent Object Reference") (OtherActor :type "Actor Object Reference") (OtherComp :type "PrimitiveComponent Object Reference") (OtherBodyIndex :type Integer) (bFromSweep :type Boolean) (SweepResult :type "HitResult Structure (by ref)"))
  ; 1. Bind to On Interact Pressed (Allow the weapon blueprint to know when the Pickup button is pressed)
  (bind _asbp_top_down_controller (cast `/Game/Characters/Player/Blueprints/BP_TopDownController` (`GameplayStatics.GetPlayerController` 0)))
  (add `/Game/Characters/Player/Blueprints/BP_TopDownController.OnPickupPressed` _asbp_top_down_controller (delegate `OnInteractWithWeapon`))
  (set `self.bOverlapWithPlayer` true))

(event `self.Sphere.OnComponentEndOverlap`
  (params (OverlappedComponent :type "PrimitiveComponent Object Reference") (OtherActor :type "Actor Object Reference") (OtherComp :type "PrimitiveComponent Object Reference") (OtherBodyIndex :type Integer))
  (set `self.bOverlapWithPlayer` false))

(event `self.ReceiveTick`
  (params (DeltaSeconds :type "Float (single-precision)"))
  (`self.K2_AddActorWorldOffset` (`KismetMathLibrary.MakeVector` 0.0 0.0 (`self.TransformedSin`))))

(fn `UserConstructionScript`)