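; BP_Sword is a pickup sword that shows a "press E to equip" text widget, removed once the player picks up a weapon.
; When its WeaponBox overlaps during an attack animation, a box trace between Start and End confirms a hit.
; A hit calls ExecuteAttack on the player's combat component, then disables the equipped sword's box collision so it only triggers once per swing.
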(event `self.ReceiveBeginPlay`
  (bind _aswbp_text (cast `/Game/Tutorial/WBP_Text` (`WidgetComponent.GetUserWidgetObject` (`self.Widget`))))
  (set `/Game/Tutorial/WBP_Text.TextValue` "Move to me and  \npress E to equip" _aswbp_text)
  (add `self.OnPlayerPickupWeapon` self (delegate `RemoveWidget`)))

(event `RemoveWidget`
  (`ActorComponent.K2_DestroyComponent` (`self.Widget`)))

(event `self.WeaponBox.OnComponentBeginOverlap`
  (params (OverlappedComponent :type "PrimitiveComponent Object Reference") (OtherActor :type "Actor Object Reference") (OtherComp :type "PrimitiveComponent Object Reference") (OtherBodyIndex :type Integer) (bFromSweep :type Boolean) (SweepResult :type "HitResult Structure (by ref)"))
  ; Player attack animation will trigger this
  ; For debugging
  (bind (_outhit _returnvalue) (`KismetSystemLibrary.BoxTraceSingle` (`SceneComponent.K2_GetComponentLocation` (`self.Start`)) (`SceneComponent.K2_GetComponentLocation` (`self.End`)) (2.5 2.5 2.5) (struct) "TraceTypeQuery1"))
  ; Execute attack when the weapon overlaps with the enemy
  (if _returnvalue
    (bind _asbp_top_down_character (cast `/Game/Characters/Player/Blueprints/BP_TopDownCharacter` (`GameplayStatics.GetPlayerPawn` 0)))
    (`/Game/GenericComponents/AC_CombatCore.Execute Attack` (`/Game/Characters/Player/Blueprints/BP_TopDownCharacter.AC_PlayerCombatCore` _asbp_top_down_character))
    (bind _equippedweapon (`/Game/Characters/Player/Blueprints/BP_TopDownCharacter.EquippedWeapon` _asbp_top_down_character))
    ; Once the weapon hit the enemy for the first time, disable the box collision
    (cast `/Game/Items/Blueprints/BP_Sword` _equippedweapon)
    (`PrimitiveComponent.SetCollisionEnabled` (`self.GetComponentByClass` _equippedweapon "/Script/Engine.BoxComponent") "NoCollision")))

(fn `UserConstructionScript`
  (`parent.UserConstructionScript`))