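; Actor component that flashes the owner's skeletal mesh when it takes damage, for the player and minions.
; On BeginPlay it creates a dynamic material instance from mesh slot 0 and binds to the owner's OnTakeAnyDamage.
; Each hit sets emissive parameters, with a separate colour and an added base colour multiplier for BP_TopDownCharacter.
; After a delay the parameters reset to zero rather than to saved original values.
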(event `self.ReceiveBeginPlay`
  (bind _returnvalue (`self.GetOwner`))
  (bind _returnvalue_2 (`Actor.GetComponentByClass` (`self.Owner`) "/Script/Engine.SkeletalMeshComponent"))
  (set `self.Owner` _returnvalue)
  (add `Actor.OnTakeAnyDamage` _returnvalue (`|CreateDelegate` :!event `DamageFlash`))
  ; Setup dynamic material instance from the Actor's skeletal mesh material(Create Dynamic Material Instance creates a runtime copy of a material that you can modify parameters on during gameplay)
  (`/Engine/EditorBlueprintResources/StandardMacros.IsValid` _returnvalue_2
    (:`Is Valid`
      (bind _returnvalue_3 (`PrimitiveComponent.CreateDynamicMaterialInstance` _returnvalue_2 0 null "None"))
      (set `self.FlashMat` _returnvalue_3))))

(event `DamageFlash`
  (params (DamagedActor :type "Actor Object Reference") (Damage :type "Float (single-precision)") (DamageType :type "DamageType Object Reference") (InstigatedBy :type "Controller Object Reference") (DamageCauser :type "Actor Object Reference"))
  (bind _flashmat (`self.FlashMat`))
  (bind _flashmat_2 (`self.FlashMat`))
  (bind _flashmat_3 (`self.FlashMat`))
  (cast `/Game/Characters/Player/Blueprints/BP_TopDownCharacter` (`self.GetOwner`)
    (:`then`
      ; Set Damage Flash for Player
      (`MaterialInstanceDynamic.SetVectorParameterValue` _flashmat_3 "EmissiveColour" (`self.FlashColourPlayer`))
      (`MaterialInstanceDynamic.SetScalarParameterValue` _flashmat_3 "EmissiveMultiplier" (`self.FlashIntensity`))
      (`MaterialInstanceDynamic.SetScalarParameterValue` _flashmat_3 "BaseColourMultiplier" (`self.BaseColourIntensityPlayer`)))
    (:`CastFailed`
      ; Set Damage Flash values for minions
      (`MaterialInstanceDynamic.SetVectorParameterValue` _flashmat_2 "EmissiveColour" (`self.FlashColourMinion`))
      (`MaterialInstanceDynamic.SetScalarParameterValue` _flashmat_2 "EmissiveMultiplier" (`self.FlashIntensity`))))
  (`KismetSystemLibrary.Delay` (`self.FlashDuration`))
  ; Return to original values
  (`MaterialInstanceDynamic.SetVectorParameterValue` _flashmat "EmissiveColour" (struct :`A` 1.0))
  (`MaterialInstanceDynamic.SetScalarParameterValue` _flashmat "EmissiveMultiplier" 0.0)
  (`MaterialInstanceDynamic.SetScalarParameterValue` _flashmat "BaseColourMultiplier" 0.0))