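; Actor component that gives AI minions a ranged attack by firing a projectile at a target actor.
; FireProjectile spawns the configured projectile class at the owner's location plus a muzzle offset, rotated to face the target's location, then sets the owner as the projectile's InstigatorActor.
; The offset is added in world space, so it does not turn with the owner.
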(fn `FireProjectile`
  (params (TargetActor :type "Actor Object Reference"))
  (bind _returnvalue (+ (`Actor.K2_GetActorLocation` (`self.GetOwner`)) (`self.MuzzleOffset`)))
  (bind _returnvalue_2 (`|SpawnActorFromClass` (`self.ProjectileClass`) (`KismetMathLibrary.MakeTransform` _returnvalue (`KismetMathLibrary.FindLookAtRotation` _returnvalue (`Actor.K2_GetActorLocation` TargetActor))) "Undefined" "MultiplyWithRoot" null null))
  (set `/Game/Characters/Minion/BP_Minion_Projectile_Base.InstigatorActor` (`self.GetOwner`) _returnvalue_2))