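; Base minion character with health, a team and an empty Attack event, acting as an AI agent that others can score and target.
; Damage updates the overhead health bar, plays a hit montage and spawns a damage popup; at zero health it waits out the death animation, then destroys itself.
; Attacker slots cap claims, and target scoring weighs health, slot occupancy and distance.
; A looping timer caches the Blackboard TargetActor, whose slot is released on death.
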(event `self.ReceiveBeginPlay`
  (set `self.Health` (`self.MaxHealth`))
  (`KismetSystemLibrary.K2_SetTimer` null "GetBBData" 0.3 true)
  (bind _aswbp_minion_health (cast `/Game/Characters/Minion/WBP_MinionHealth` (`WidgetComponent.GetUserWidgetObject` (`self.HealthBarComponent`))))
  (set `/Game/Characters/Minion/WBP_MinionHealth.Name` (`self.Name`) _aswbp_minion_health)
  (set `/Game/Characters/Minion/WBP_MinionHealth.CurrentHP` (`self.Health`) _aswbp_minion_health)
  (set `/Game/Characters/Minion/WBP_MinionHealth.MaxHP` (`self.MaxHealth`) _aswbp_minion_health)
  (`/Game/Characters/Minion/WBP_MinionHealth.UpdateHPBar` _aswbp_minion_health))

(event `/Game/GenericComponents/BPI_Attackable.Attack`
  (params (Targett :type "Actor Object Reference")))

(event `self.ReceiveAnyDamage`
  (params (Damage :type "Float (single-precision)") (DamageType :type "DamageType Object Reference") (InstigatedBy :type "Controller Object Reference") (DamageCauser :type "Actor Object Reference"))
  ; Take Damage
  (`|ExecutionSequence`
    (:`then_0`
      (set `self.Health` (- (`self.Health`) Damage))
      (`KismetSystemLibrary.PrintString` (`KismetStringLibrary.Concat_StrStr` "Ouch, I got hit! HP Left: " (`KismetStringLibrary.Conv_DoubleToString` (`self.Health`))))
      ;; Play animation for getting hit
      (`self.PlayAnimMontage` (`self.GetHitAnimMontage`)))
    (:`then_1`
      (`|SpawnActorFromClass` "/Game/Characters/Minion/BP_DamagePopUp.BP_DamagePopUp_C" (`KismetMathLibrary.MakeTransform` (+ (`self.K2_GetActorLocation`) (0.0 0.0 160.0))) "Undefined" "MultiplyWithRoot" null (`KismetTextLibrary.Conv_DoubleToText` Damage "HalfToEven") null))
    (:`then_2`
      (bind _aswbp_minion_health (cast `/Game/Characters/Minion/WBP_MinionHealth` (`WidgetComponent.GetUserWidgetObject` (`self.HealthBarComponent`))))
      (set `/Game/Characters/Minion/WBP_MinionHealth.CurrentHP` (`self.Health`) _aswbp_minion_health)
      (set `/Game/Characters/Minion/WBP_MinionHealth.MaxHP` (`self.MaxHealth`) _aswbp_minion_health)
      (`/Game/Characters/Minion/WBP_MinionHealth.UpdateHPBar` _aswbp_minion_health))
    (:`then_3`
      (if (<= (`self.Health`) 0.0)
        (`self.SetMinionState` "EMS_Dead")
        ;; Time taken for the death animation
        (`KismetSystemLibrary.Delay` (+ (`AnimationAsset.GetPlayLength` (`self.DeathAnimSequence`)) 0.5))
        (`self.Handle Death`)))))

(event `/Game/GenericComponents/BPI_TeamAgent.ReleaseSlot`
  ; ReleaseSlot
  (if (> (`self.CurrentSlots`) 0.0)
    (set `self.CurrentSlots` (- (`self.CurrentSlots`) 1.0))))

(fn `CalculateTargetScore`
  (params (AttackerLocation :type "Vector Structure"))
  (returns (TargetScore :type "Float (double-precision)"))
  (locals (FinalScore :type "Float (double-precision)"))
  (bind _returnvalue (/ (`self.CurrentSlots`) (`self.MaxSlot`)))
  (bind _returnvalue_2 (/ (`self.Health`) (`self.MaxHealth`)))
  (`|ExecutionSequence`
    (:`then_0`
      ; Check Health
      (if (< _returnvalue_2 0.3)
        (set `local.FinalScore` (+ (`local.FinalScore`) 50.0))
        (elif (< _returnvalue_2 0.7)
          (set `local.FinalScore` (+ (`local.FinalScore`) 30.0))
          (else
            (set `local.FinalScore` (+ (`local.FinalScore`) 10.0))))))
    (:`then_1`
      ; Check Slot
      (if (< _returnvalue 0.2)
        (set `local.FinalScore` (+ (`local.FinalScore`) 50.0))
        (elif (> _returnvalue 1.0)
          (set `local.FinalScore` (+ (`local.FinalScore`) 0.0))
          (else
            (set `local.FinalScore` (+ (`local.FinalScore`) 20.0))))))
    (:`then_2`
      ; Check Distance
      (set `local.FinalScore` (- (`local.FinalScore`) (/ (`KismetMathLibrary.Vector_Distance` AttackerLocation (`self.K2_GetActorLocation`)) 100.0))))
    (:`then_3`
      ; Output
      (return (`local.FinalScore`)))))

(fn `ClaimSlot`
  (returns (canClaim :type Boolean))
  (bind _canclaim (`self.HasOpenSlot`))
  (if _canclaim
    (set `self.CurrentSlots` (+ (`self.CurrentSlots`) 1.0))
    (return true)
    (else
      (return false))))

(fn `get Team`
  (returns (Team :type "/Game/GenericComponents/ETeam Enum"))
  (return (`self.Team`)))

(fn `GetBBData`
  (bind _returnvalue (`BlackboardComponent.GetValueAsObject` (`AIBlueprintHelperLibrary.GetBlackboard` null) "TargetActor"))
  (bind _asactor (cast `Actor` _returnvalue)
    (:`then`
      (set `self.TargetActor` _asactor)
      (`KismetSystemLibrary.PrintString` (`KismetStringLibrary.Concat_StrStr` "TargetActor: " (`KismetSystemLibrary.GetDisplayName` _returnvalue)) false))
    (:`CastFailed`
      (set `self.TargetActor` null))))

(fn `Handle Death`
  (bind _asbpi_team_agent (cast `/Game/GenericComponents/BPI_TeamAgent` (`self.TargetActor`))
    (:`then`
      (`/Game/GenericComponents/BPI_TeamAgent.ReleaseSlot` _asbpi_team_agent))
    (:`CastFailed`
      _))
  (set `self.isDead` true)
  (`self.K2_DestroyActor`))

(fn `HasOpenSlot`
  (returns (canClaim :type Boolean))
  (if (< (`self.CurrentSlots`) (`self.MaxSlot`))
    (return true)
    (else
      (return false))))

(fn `UserConstructionScript`)