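; BP_Friendly_Range is a friendly ranged minion that sets its death animation and get-hit montage on BeginPlay.
; Its Attack event checks that the target is valid and the minion is not dead, plays the attack montage, then calls TryAttack on the ranged combat component after a short delay.
; Interaction is delegated to a follow-on-interact component, and an event applies overlay materials to the mesh.
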(event `self.ReceiveBeginPlay`
  (`parent.ReceiveBeginPlay`)
  (set `self.DeathAnimSequence` "/Game/MonsterForSurvivalGame/Animation/Polyart/Swarm08/Swarm08_Die_Anim.Swarm08_Die_Anim")
  (set `self.GetHitAnimMontage` "/Game/Characters/Minion/Friendly/Ranged/AM_GetHit.AM_GetHit"))

(event `/Game/GenericComponents/BPI_Attackable.Attack`
  (params (Targett :type "Actor Object Reference"))
  (`/Engine/EditorBlueprintResources/StandardMacros.IsValid` Targett
    (:`Is Valid`
      ; Prevent attacking when dead
      (if (`|EnumInequality` (`self.GetMinionState`) "EMS_Dead")
        (`self.PlayAnimMontage` "/Game/Characters/Minion/Friendly/Ranged/AM_Attack.AM_Attack")
        (`KismetSystemLibrary.Delay` 0.5)
        (`/Game/GenericComponents/AC_CombatCore.Try Attack` (`self.AC_AIRangedCombat`) Targett)))))

(event `/Game/GenericComponents/BPI_Interactable.BeInteractedWith`
  (params (Interactor :type "Actor Object Reference"))
  (`/Game/Characters/Minion/AC_FollowOnInteract.Handle Interact` (`self.AC_FollowOnInteract`) Interactor))

(event `UpdateOverlayMaterial`
  (params (OverlayMaterial :type "MaterialInstance Object Reference"))
  (`MeshComponent.SetOverlayMaterial` (`self.Mesh`) OverlayMaterial))

(fn `UserConstructionScript`
  (`parent.UserConstructionScript`))