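; Abstract base for friendly minions that follow a blackboard Leader as a swarm, using steering forces.
; A looping timer gathers nearby minions, reads the Leader, and pathfinds to it for the next waypoint, clearing the follow target while TargetActor is valid.
; Tick sums separation, curve-weighted goal pull and a randomly biased sideways orbit when those two oppose, feeds the result to movement input, and draws debug arrows.
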(event `self.ReceiveBeginPlay`
  (`parent.ReceiveBeginPlay`)
  (`|ExecutionSequence`
    (:`then_0`
      (`KismetSystemLibrary.K2_SetTimer` null "GetNavigationData" 0.3 true))
    (:`then_1`
      (if (`KismetMathLibrary.RandomBool`)
        (set `self.OrbitDirectionBias` 1.0)
        (else
          (set `self.OrbitDirectionBias` -1.0))))))

(event `self.ReceiveTick`
  (params (DeltaSeconds :type "Float (single-precision)"))
  (`parent.ReceiveTick` DeltaSeconds)
  (`self.CalculateStreeringForce`))

(fn `CalculateStreeringForce`
  (locals (V_Avoid :type "Vector Structure") (V_Sep :type "Vector Structure") (V_Goal :type "Vector Structure") (V_Orbit :type "Vector Structure") (BaseDirection :type "Vector Structure") (CurveWeight :type "Float (double-precision)") (DistanceToGoalBuffer :type "Float (double-precision)"))
  (bind _returnvalue (`self.K2_GetActorLocation`))
  (bind _returnvalue_2 (`self.K2_GetActorLocation`))
  (bind _returnvalue_3 (`self.K2_GetActorLocation`))
  (bind _returnvalue_4 (`self.K2_GetActorLocation`))
  (bind _returnvalue_5 (`KismetMathLibrary.Dot_VectorVector` (`local.V_Sep`) (`local.V_Goal`)))
  (bind _returnvalue_6 (`KismetMathLibrary.Normal` (* (- (`self.CurrentWaypoint`) _returnvalue) (1.0 1.0 0.0))))
  (bind _returnvalue_7 (`CurveFloat.GetFloatValue` (`self.FuzzyCurve`) (- (`KismetMathLibrary.VSize` (- (`self.K2_GetActorLocation` (`self.FollowTarget`)) _returnvalue)) (`local.DistanceToGoalBuffer`))))
  (if (== (`self.Leader`) (`self.FollowTarget`))
    (set `local.DistanceToGoalBuffer` (`self.LeashLength`))
    (else
      (set `local.DistanceToGoalBuffer` (`self.AttackRange`))))
  (`|ExecutionSequence`
    (:`then_0`
      ; Agent Separation
      (set `local.V_Sep` (0.0 0.0 0.0))
      (for _array_element (`self.NearbyMinions`)
        (`/Engine/EditorBlueprintResources/StandardMacros.IsValid` _array_element
          (:`Is Valid`
            (bind _returnvalue_8 (- (`self.K2_GetActorLocation`) (`self.K2_GetActorLocation` _array_element)))
            (set `local.V_Sep` (+ (`local.V_Sep`) (* (`KismetMathLibrary.Normal` _returnvalue_8) (`KismetMathLibrary.MapRangeClamped` (`KismetMathLibrary.VSize` _returnvalue_8) 0.0 (`self.NearbyMinionRange`) 10.0))))))))
    (:`then_1`
      ; Agent Goal
      (`/Engine/EditorBlueprintResources/StandardMacros.IsValid` (`self.FollowTarget`)
        (:`Is Valid`
          (set `local.BaseDirection` _returnvalue_6)
          (set `local.CurveWeight` _returnvalue_7)
          (set `local.V_Goal` (* _returnvalue_6 _returnvalue_7)))))
    (:`then_2`
      ; Agent Orbit
      (if (< _returnvalue_5 0.0)
        (set `local.V_Orbit` (* (* (* (`KismetMathLibrary.Normal` (`KismetMathLibrary.Cross_VectorVector` (`local.BaseDirection`) (0.0 0.0 1.0))) (- 1.0 (`local.CurveWeight`))) (`self.OrbitDirectionBias`)) _returnvalue_5))
        (else
          (set `local.V_Orbit` (0.0 0.0 0.0)))))
    (:`then_3`
      ; Final Movement
      (`self.AddMovementInput` (+ (`local.V_Sep`) (`local.V_Goal`) (`local.V_Orbit`))))
    (:`then_4`
      ; Arrow Debyg
      (`KismetSystemLibrary.DrawDebugArrow` _returnvalue_3 (+ _returnvalue_3 (* (`local.V_Sep`) 100.0)) 0.5 (struct :`R` 0.354167 :`G` 0.044091 :`B` 0.035569 :`A` 1.0) 0.1 1.0)
      (`KismetSystemLibrary.DrawDebugArrow` _returnvalue_4 (+ _returnvalue_4 (* (`local.V_Goal`) 150.0)) 1.0 (struct :`R` 1.0 :`G` 0.826263 :`A` 1.0) 0.1 3.0)
      (`KismetSystemLibrary.DrawDebugArrow` _returnvalue_2 (+ _returnvalue_2 (* (`local.V_Orbit`) 100.0)) 0.5 (struct :`R` 0.240669 :`G` 0.152639 :`B` 1.0 :`A` 1.0) 0.1 1.0))))

(fn `get Team`
  (returns (Team :type "/Game/GenericComponents/ETeam Enum"))
  (return (`self.Team`)))

(fn `GetNavigationData`
  (bind _returnvalue (`self.K2_GetActorLocation`))
  (bind _leader (`self.Leader`))
  (bind _followtarget (`self.FollowTarget`))
  (bind _returnvalue_2 (`BlackboardComponent.GetValueAsObject` (`AIBlueprintHelperLibrary.GetBlackboard` null) "Leader"))
  (`|ExecutionSequence`
    (:`then_0`
      ; Get Nearby Friendly Minions
      (bind _outactors (`KismetSystemLibrary.SphereOverlapActors` (`self.K2_GetActorLocation`) (`self.NearbyMinionRange`) (`|MakeArray` "ObjectTypeQuery3" :!type "EObjectTypeQuery Enum") "BP_FriendlyMinionCharacter_Abstract_C" (`|MakeArray` (`GameplayStatics.GetPlayerPawn` 0) self :!type "Actor Object Reference")))
      (set `self.NearbyMinions` _outactors))
    (:`then_2`
      ; Update Leader from BlackBoard
      (bind _asactor (cast `Actor` _returnvalue_2)
        (:`then`
          (set `self.Leader` _asactor)
          (`KismetSystemLibrary.PrintString` (`KismetStringLibrary.Concat_StrStr` "Leader:" (`KismetSystemLibrary.GetDisplayName` _returnvalue_2)) false))
        (:`CastFailed`
          (set `self.Leader` null))))
    (:`then_3`
      ; Set Follow Target = TargetActor > Leader
      (`/Engine/EditorBlueprintResources/StandardMacros.IsValid` (`self.TargetActor`)
        (:`Is Valid`
          (set `self.FollowTarget` null))
        (:`Is Not Valid`
          (`/Engine/EditorBlueprintResources/StandardMacros.IsValid` _leader
            (:`Is Valid`
              (set `self.FollowTarget` _leader))
            (:`Is Not Valid`
              (set `self.FollowTarget` null))))))
    (:`then_4`
      ; Pathingfinding with swarm navigation
      (`/Engine/EditorBlueprintResources/StandardMacros.IsValid` _followtarget
        (:`Is Valid`
          (bind _returnvalue_3 (`NavigationSystemV1.FindPathToActorSynchronously` _returnvalue _followtarget (`self.LeashLength`) null null))
          (bind _pathpoints (`NavigationPath.PathPoints` _returnvalue_3))
          (bind _returnvalue_4 (`KismetArrayLibrary.Array_Length` _pathpoints))
          (if (> _returnvalue_4 1)
            (bind _output (`|GetArrayItem` _pathpoints 1))
            (if (< (`KismetMathLibrary.Vector_Distance` (`self.K2_GetActorLocation`) _output) 100.0)
              (if (> _returnvalue_4 2)
                (set `self.CurrentWaypoint` (`|GetArrayItem` _pathpoints 2))
                (else
                  (set `self.CurrentWaypoint` _output :!label _label)))
              (else
                (goto _label)))
            (else
              (set `self.CurrentWaypoint` (`self.K2_GetActorLocation` (`self.FollowTarget`))))))
        (:`Is Not Valid`
          (set `self.CurrentWaypoint` _returnvalue))))))

(fn `UserConstructionScript`
  (`parent.UserConstructionScript`))