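; Friendly melee minion character, a child Blueprint that sets its own mushroom death animation and hit montage and reports a fixed team.
; Attack plays the attack montage, waits out its length, then rechecks the target, turns to face it and calls the AI melee attack component.
; Interaction is forwarded to the follow-on-interact component.
; A dead-state check meant to block attacks is left unconnected.
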(event `self.ReceiveBeginPlay`
  (`parent.ReceiveBeginPlay`)
  (set `self.DeathAnimSequence` "/Game/MonsterForSurvivalGame/Animation/Polyart/Mushroom/SmileVersion/Mushroom_DieSmile_ANIM.Mushroom_DieSmile_ANIM")
  (set `self.GetHitAnimMontage` "/Game/Characters/Minion/Friendly/Melee/AM_GetHit.AM_GetHit"))

(event `/Game/GenericComponents/BPI_Attackable.Attack`
  (params (Target :type "Actor Object Reference"))
  (`/Engine/EditorBlueprintResources/StandardMacros.IsValid` Target
    (:`Is Valid`
      (`self.PlayAnimMontage` "/Game/Characters/Minion/Friendly/Melee/AM_AttackMontage.AM_AttackMontage")
      (`KismetSystemLibrary.Delay` (`AnimationAsset.GetPlayLength` (`self.GetCurrentMontage`)))
      (`/Engine/EditorBlueprintResources/StandardMacros.IsValid` Target
        (:`Is Valid`
          (`self.K2_SetActorRotation` self (`KismetMathLibrary.FindLookAtRotation` (`self.K2_GetActorLocation` self) (`self.K2_GetActorLocation` Target)) false)
          (`/Game/GenericComponents/AC_CombatCore.Try Attack` (`self.AC_AIMeleeAttack`) Target))))))

(event `/Game/GenericComponents/BPI_Interactable.BeInteractedWith`
  (params (Interactor :type "Actor Object Reference"))
  (`/Game/Characters/Minion/AC_FollowOnInteract.Handle Interact` (`self.AC_FollowOnInteract`) Interactor))

(fn `get Team`
  (returns (Team :type "/Game/GenericComponents/ETeam Enum"))
  (return "NewEnumerator0"))

(fn `UserConstructionScript`
  (`parent.UserConstructionScript`))