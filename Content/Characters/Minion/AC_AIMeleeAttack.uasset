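; Actor component that gives an AI minion a melee attack.
; ExecuteAttack runs a sphere overlap for pawns at a point in front of the owning character, ignoring the owner, and applies damage to the actors it finds.
; Friendly fire is filtered by comparing each target's team, read through BPI_TeamAgent, with the owning minion's team.
; The attack also prints a debug string.
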(fn `Execute Attack`
  (locals (`Attack Center` :type "Vector Structure"))
  (bind _owning_character (`self.Owning Character`))
  (`KismetSystemLibrary.PrintString` "Enemy Minion Attacking")
  (bind _output_get (set `local.Attack Center` (+ (`Actor.K2_GetActorLocation` _owning_character) (* (`Actor.GetActorForwardVector` _owning_character) (`self.Attack Range`)))))
  (bind _outactors (`KismetSystemLibrary.SphereOverlapActors` _output_get (`self.Attack Radius`) (`|MakeArray` "ObjectTypeQuery3" :!type "EObjectTypeQuery Enum") null (`|MakeArray` (`self.Owning Character`) :!type "Actor Object Reference")))
  (for _array_element _outactors
    (bind _asbpi_team_agent (cast `/Game/GenericComponents/BPI_TeamAgent` _array_element))
    ; Friendly Fire Detection
    (bind _team (`/Game/GenericComponents/BPI_TeamAgent.get Team` _asbpi_team_agent))
    (bind _asbp_base_minion_character_abstract (cast `/Game/Characters/Minion/BP_BaseMinionCharacter_Abstract` (`self.Owning Character`)))
    (bind _team_2 (`/Game/GenericComponents/BPI_TeamAgent.get Team` _asbp_base_minion_character_abstract))
    (if (not (`|EnumEquality` _team _team_2))
      (`GameplayStatics.ApplyDamage` _array_element (`self.Base Damage`) (`Pawn.GetController` _asbp_base_minion_character_abstract) _asbp_base_minion_character_abstract))))