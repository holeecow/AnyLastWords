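; Actor component for minion characters that makes the owning minion follow whoever interacts with it.
; HandleInteract caches the owning minion, flags it as following, and gets its generic minion AI controller's blackboard.
; It writes the interacting actor to the Leader key and stores a friendly-minion outline material in the OverlayMaterial key, leaving the behavior to the AI.
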(fn `Handle Interact`
  (params (`Interacting Actor` :type "Actor Object Reference"))
  (locals (`Owner Minion` :type "/Game/Characters/Minion/BP_BaseMinionCharacter_Abstract Object Reference") (`Blackboard Component` :type "BlackboardComponent Object Reference") (NewLocalVar :type "Actor Object Reference"))
  (bind _blackboard_component (`local.Blackboard Component`))
  (bind _asbp_base_minion_character_abstract (cast `/Game/Characters/Minion/BP_BaseMinionCharacter_Abstract` (`self.GetOwner`)))
  (bind _output_get (set `local.Owner Minion` _asbp_base_minion_character_abstract))
  (set `self.isFollowing` true)
  (bind _asaic_generic_minion (cast `/Game/Characters/Minion/AIC_GenericMinion` (`Pawn.GetController` _output_get)))
  (set `local.Blackboard Component` (`AIController.Blackboard` _asaic_generic_minion))
  (if (`self.isFollowing`)
    (`BlackboardComponent.SetValueAsObject` _blackboard_component "Leader" `Interacting Actor`)
    (`BlackboardComponent.SetValueAsObject` _blackboard_component "OverlayMaterial" "/Game/Characters/Minion/Materials/M_Outline_FriendlyMinion.M_Outline_FriendlyMinion")))