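; Melee enemy minion character that attacks a given target on its Attack event.
; When the target is valid, the event asks the ACAIMeleeAttack component to try the attack.
; On success, it snaps the actor's rotation toward the target and plays one of two attack montages at random.
; BeginPlay, overlap and Tick are disabled stubs, and the construction script only calls the parent.
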(event `/Game/GenericComponents/BPI_Attackable.Attack`
  (params (Targett :type "Actor Object Reference"))
  (`/Engine/EditorBlueprintResources/StandardMacros.IsValid` Targett
    (:`Is Valid`
      (bind _issucessful (`/Game/GenericComponents/AC_CombatCore.Try Attack` (`self.AC_AIMeleeAttack`) Targett))
      (if _issucessful
        (`self.K2_SetActorRotation` self (`KismetMathLibrary.FindLookAtRotation` (`self.K2_GetActorLocation` self) (`self.K2_GetActorLocation` Targett)) false)
        (`self.PlayAnimMontage` (`KismetArrayLibrary.Array_Random` (`|MakeArray` "/Game/Characters/Player/Anims/Unarmed/Attack/AM_Attack_01_Montage.AM_Attack_01_Montage" "/Game/Characters/Player/Anims/Unarmed/Attack/AM_Attack_02_Montage.AM_Attack_02_Montage" :!type "AnimMontage Object Reference")))))))

(fn `UserConstructionScript`
  (`parent.UserConstructionScript`))