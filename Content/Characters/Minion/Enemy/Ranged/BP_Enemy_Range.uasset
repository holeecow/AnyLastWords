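; Ranged enemy minion character that supplies its own attack behavior and reports a fixed team through Get Team.
; The Attack event checks that the target is valid, plays the attack montage, then waits briefly before passing the target to the AI ranged combat component's TryAttack.
; The fixed delay, rather than an anim notify, times the attack against the animation, and target validity is not rechecked afterward in this Blueprint.
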(event `/Game/GenericComponents/BPI_Attackable.Attack`
  (params (Targett :type "Actor Object Reference"))
  (`/Engine/EditorBlueprintResources/StandardMacros.IsValid` Targett
    (:`Is Valid`
      (`self.PlayAnimMontage` "/Game/Characters/Minion/Enemy/Ranged/AM_AttackMontage.AM_AttackMontage")
      (`KismetSystemLibrary.Delay` 0.5)
      (`/Game/GenericComponents/AC_CombatCore.Try Attack` (`self.AC_AIRangedCombat`) Targett))))

(fn `get Team`
  (returns (Team :type "/Game/GenericComponents/ETeam Enum"))
  (return "NewEnumerator1"))

(fn `UserConstructionScript`
  (`parent.UserConstructionScript`))