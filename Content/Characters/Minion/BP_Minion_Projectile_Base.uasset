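; Base projectile for minion attacks that damages actors on other teams.
; Activates its projectile movement on BeginPlay.
; On sphere overlap, it compares the team of the hit actor, read through BPI_TeamAgent, with that of the instigating minion character.
; A differing team takes damage credited to that minion and its controller, then the projectile destroys itself; teammates and non-team actors are ignored.
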(event `self.ReceiveBeginPlay`
  (`ActorComponent.Activate` (`self.ProjectileMovement`) false))

(event `self.Sphere1.OnComponentBeginOverlap`
  (params (OverlappedComponent :type "PrimitiveComponent Object Reference") (OtherActor :type "Actor Object Reference") (OtherComp :type "PrimitiveComponent Object Reference") (OtherBodyIndex :type Integer) (bFromSweep :type Boolean) (SweepResult :type "HitResult Structure (by ref)"))
  (bind _asbpi_team_agent (cast `/Game/GenericComponents/BPI_TeamAgent` OtherActor))
  ; Friendly Fire Detection
  (bind _team (`/Game/GenericComponents/BPI_TeamAgent.get Team` _asbpi_team_agent))
  (bind _asbp_base_minion_character_abstract (cast `/Game/Characters/Minion/BP_BaseMinionCharacter_Abstract` (`self.InstigatorActor`)))
  (bind _team_2 (`/Game/GenericComponents/BPI_TeamAgent.get Team` _asbp_base_minion_character_abstract))
  (if (not (`|EnumEquality` _team _team_2))
    (`GameplayStatics.ApplyDamage` OtherActor (`self.Damage`) (`Pawn.GetController` _asbp_base_minion_character_abstract) _asbp_base_minion_character_abstract)
    (`self.K2_DestroyActor`)))

(fn `UserConstructionScript`)