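; Boss character with a health bar, weighted random attacks, and a death that opens the JudasDeath level.
; Attack picks tower spawn, minion spawn or most often jump AoE, setting the current attack component and pausing the behavior tree during its montage.
; Damage plays a hit reaction, spawns a popup and updates the bar.
; Reset plays a montage, moves it home, clears target sight and restarts AI; targeting functions return fixed values.
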(event `self.ReceiveBeginPlay`
  (set `self.AttackArray` (`|MakeArray` (`self.AC_Attack_JumpAoE`) (`self.AC_Attack_SpawnMinion`) (`self.AC_Attack_SpawnTower`) :!type "/Game/Characters/Boss/AC_BossAttackBase Object Reference"))
  (set `self.Health` (`self.MaxHealth`))
  (bind _returnvalue (`|CreateWidget` "/Game/Characters/Minion/WBP_MinionHealth.WBP_MinionHealth_C" null (`self.Health`) (`self.MaxHealth`) (`self.Name`) (`self.HealthColor`) 100.0))
  (`WidgetComponent.SetWidget` (`self.HealthBarComponent`) _returnvalue)
  (`/Game/Characters/Minion/WBP_MinionHealth.UpdateHPBar` _returnvalue)
  (`/Game/Characters/Minion/WBP_MinionHealth.UpdateStyling` _returnvalue)
  (set `self.Home Location` (`self.K2_GetActorLocation`)))

(event `/Game/GenericComponents/BPI_Attackable.Attack`
  (params (Target :type "Actor Object Reference"))
  (bind _returnvalue (`AIBlueprintHelperLibrary.GetAIController` self))
  (if (not (`self.isAttacking`))
    (set `self.RNGValue` (`KismetMathLibrary.RandomFloatInRange` 0.0 100.0))
    (if (<= (`self.RNGValue`) 10.0)
      (set `self.currentAttack` (`self.AC_Attack_SpawnTower`))
      (set `self.AttackMontageToPlay` "/Game/Characters/Boss/Anim/AM_SpawnTower_Boss.AM_SpawnTower_Boss")
      (set `self.Montage Play Speed` 0.65)
      (elif (<= (`self.RNGValue`) 40.0)
        (set `self.currentAttack` (`self.AC_Attack_SpawnMinion`))
        (set `self.AttackMontageToPlay` "/Game/Characters/Boss/Anim/AM_SpawnMinion_Boss.AM_SpawnMinion_Boss")
        (set `self.Montage Play Speed` 0.65)
        (else
          (set `self.currentAttack` (`self.AC_Attack_JumpAoE`))
          (set `self.AttackMontageToPlay` "/Game/Characters/Boss/Anim/AM_JumpAoE_Boss.AM_JumpAoE_Boss")
          (set `self.Montage Play Speed` 0.3))))
    (`|PlayMontage` (`self.Mesh`) (`self.AttackMontageToPlay`) (`self.Montage Play Speed`)
      (:`then`
        (`BrainComponent.StopLogic` (`AIController.BrainComponent` _returnvalue) "")
        (set `self.isAttacking` true))
      (:`OnCompleted`
        (`AIController.RunBehaviorTree` _returnvalue "/Game/Characters/Boss/BT_Boss.BT_Boss")
        (set `self.isAttacking` false)))))

(event `self.ReceiveAnyDamage`
  (params (Damage :type "Float (single-precision)") (DamageType :type "DamageType Object Reference") (InstigatedBy :type "Controller Object Reference") (DamageCauser :type "Actor Object Reference"))
  ; Take Damage
  (`|ExecutionSequence`
    (:`then_0`
      (set `self.Health` (- (`self.Health`) Damage))
      (`KismetSystemLibrary.PrintString` (`KismetStringLibrary.Concat_StrStr` "Boss got hit! HP Left: " (`KismetStringLibrary.Conv_DoubleToString` (`self.Health`))))
      ;; Play animation for getting hit
      (`self.PlayAnimMontage` (`self.GetHitAnimMontage`)))
    (:`then_1`
      (`|SpawnActorFromClass` "/Game/Characters/Minion/BP_DamagePopUp.BP_DamagePopUp_C" (`KismetMathLibrary.MakeTransform` (+ (`self.K2_GetActorLocation`) (0.0 0.0 160.0))) "Undefined" "MultiplyWithRoot" null (`KismetTextLibrary.Conv_DoubleToText` Damage "HalfToEven") (`self.HealthColor`) null))
    (:`then_2`
      (bind _aswbp_minion_health (cast `/Game/Characters/Minion/WBP_MinionHealth` (`WidgetComponent.GetUserWidgetObject` (`self.HealthBarComponent`))))
      (set `/Game/Characters/Minion/WBP_MinionHealth.CurrentHP` (`self.Health`) _aswbp_minion_health)
      (set `/Game/Characters/Minion/WBP_MinionHealth.MaxHP` (`self.MaxHealth`) _aswbp_minion_health)
      (`/Game/Characters/Minion/WBP_MinionHealth.UpdateHPBar` _aswbp_minion_health))
    (:`then_3`
      (if (<= (`self.Health`) 0.0)
        (`CharacterMovementComponent.DisableMovement` (`self.CharacterMovement`))
        (`BrainComponent.StopLogic` (`AIController.BrainComponent` (`AIBlueprintHelperLibrary.GetAIController` self)) "")
        (`|PlayMontage` null "/Game/Characters/Boss/Anim/AM_Die_Boss.AM_Die_Boss"
          (:`then`
            (`KismetSystemLibrary.Delay` 0.8)
            (`GameplayStatics.OpenLevel` "Lvl_JudasDeath")))))))

(event `resetToBase`
  (bind _returnvalue (`AIBlueprintHelperLibrary.GetAIController` self))
  (`BrainComponent.StopLogic` (`AIController.BrainComponent` _returnvalue) "")
  (bind _returnvalue_2 (`self.PlayAnimMontage` "/Game/Characters/Boss/Anim/AM_ResetToBase_Boss.AM_ResetToBase_Boss" 0.3))
  (`KismetSystemLibrary.Delay` (/ _returnvalue_2 0.3))
  (`self.K2_SetActorLocation` (`self.Home Location`))
  (`BlackboardComponent.SetValueAsBool` (`AIBlueprintHelperLibrary.GetBlackboard` _returnvalue) "canSeeTarget" false)
  (`AIController.RunBehaviorTree` _returnvalue "/Game/Characters/Boss/BT_Boss.BT_Boss"))

(fn `CalculateTargetScore`
  (params (AttackerLocation :type "Vector Structure"))
  (returns (TargetScore :type "Float (double-precision)"))
  (return 20000.0))

(fn `ClaimSlot`
  (returns (canClaim :type Boolean))
  (return false))

(fn `get Team`
  (returns (Team :type "/Game/GenericComponents/ETeam Enum"))
  (return "NewEnumerator1"))

(fn `HasOpenSlot`
  (returns (canClaim :type Boolean))
  (return true))

(fn `UserConstructionScript`)