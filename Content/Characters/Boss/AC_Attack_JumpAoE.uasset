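; AC_Attack_JumpAoE is a boss attack component that deals radial area damage around its owner, with no jump movement in this graph.
; ExecuteAttack sphere-overlaps pawns and dynamic world objects within Radius of the owner, ignoring the owner, and prints a debug string.
; Hit actors implementing BPI_TeamAgent take Damage unless their team matches one hardcoded enum value, which serves as the friendly-fire filter.
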(fn `ExecuteAttack`
  (locals (`Owning Actor` :type "Actor Object Reference"))
  (set `local.Owning Actor` (`self.GetOwner`))
  (`KismetSystemLibrary.PrintString` "Boss Jump AoE")
  (bind _outactors (`KismetSystemLibrary.SphereOverlapActors` (`Actor.K2_GetActorLocation` (`local.Owning Actor`)) (`self.Radius`) (`|MakeArray` "ObjectTypeQuery3" "ObjectTypeQuery2" :!type "EObjectTypeQuery Enum") null (`|MakeArray` (`local.Owning Actor`))))
  (for _array_element _outactors
    (bind _asbpi_team_agent (cast `/Game/GenericComponents/BPI_TeamAgent` _array_element))
    ; Friendly Fire Detection
    (bind _team (`/Game/GenericComponents/BPI_TeamAgent.get Team` _asbpi_team_agent))
    (if (not (`|EnumEquality` _team "NewEnumerator1"))
      (`GameplayStatics.ApplyDamage` _array_element (`self.Damage`)))))