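; Boss attack component that summons enemy towers around its owner, up to a maximum count.
; ExecuteAttack makes a weighted random roll to pick one of four tower classes, then always spawns it at the location from FindValidSpawnLocation.
; That function picks a random angle and distance around the owner at its height, with no ground or overlap check.
; The spawn counter only increases here, so destroyed towers do not free up slots.
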(fn `ExecuteAttack`
  (locals (TowerToSummon :type "/Game/Towers/BP_TowerBase Class Reference") (RNGValue :type "Float (double-precision)" :default 0.0) (OwningActor :type "Actor Object Reference"))
  (set `local.OwningActor` (`self.GetOwner`))
  (if (< (`self.SpawnTowerCount`) (`self.MaxSpawnedTowers`))
    (`KismetSystemLibrary.PrintString` "Boss summons tower")
    (set `local.RNGValue` (`KismetMathLibrary.RandomFloatInRange` 0.0 100.0))
    (if (<= (`local.RNGValue`) 10.0)
      (set `local.TowerToSummon` "/Game/Towers/BP_BossTower.BP_BossTower_C")
      (elif (<= (`local.RNGValue`) 60.0)
        (set `local.TowerToSummon` "/Game/Towers/BP_TowerShuriken.BP_TowerShuriken_C")
        (elif (<= (`local.RNGValue`) 80.0)
          (set `local.TowerToSummon` "/Game/Towers/BP_TowerBoomerang.BP_TowerBoomerang_C")
          (else
            (set `local.TowerToSummon` "/Game/Towers/BP_TowerFuzzBall.BP_TowerFuzzBall_C")))))
    (bind _spawnlocation (`self.FindValidSpawnLocation`))
    (`|SpawnActorFromClass` (`local.TowerToSummon`) (`KismetMathLibrary.Conv_VectorToTransform` _spawnlocation) "AlwaysSpawn" "MultiplyWithRoot" null null)
    (set `self.SpawnTowerCount` (+ (`self.SpawnTowerCount`) 1))))

(fn `FindValidSpawnLocation`
  (returns (SpawnLocation :type "Vector Structure"))
  (locals (RandomAngle :type Integer :default 0) (RandomDistance :type Integer :default 0) (OffsetX :type "Float (double-precision)") (OffsetY :type "Float (double-precision)") (OwningActor :type "Actor Object Reference") (OwnerLocation :type "Vector Structure" :default (0.0 0.0 0.0)) (CandidateLocation :type "Vector Structure"))
  (set `local.RandomAngle` (`KismetMathLibrary.RandomIntegerInRange` 0 360))
  (set `local.RandomDistance` (`KismetMathLibrary.RandomIntegerInRange` 200 2000))
  (set `local.OffsetX` (* (`KismetMathLibrary.DegCos` (`KismetMathLibrary.Conv_IntToDouble` (`local.RandomAngle`))) (`local.RandomDistance`)))
  (set `local.OffsetY` (* (`KismetMathLibrary.DegSin` (`KismetMathLibrary.Conv_IntToDouble` (`local.RandomAngle`))) (`local.RandomDistance`)))
  (set `local.OwningActor` (`self.GetOwner`))
  (set `local.OwnerLocation` (`Actor.K2_GetActorLocation` (`local.OwningActor`)))
  (bind _output_get (set `local.CandidateLocation` (+ (`local.OwnerLocation`) (`KismetMathLibrary.MakeVector` (`local.OffsetX`) (`local.OffsetY`)))))
  (return _output_get))