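; Player actor component for ranged weapons that fires a projectile at a given target actor.
; FireProjectile spawns ProjectileClass at the owner's location plus MuzzleOffset, added without rotation, and aims it at the target's location with a look-at rotation.
; The spawn passes no owner or instigator, and a node that would set InstigatorActor to the owner is left unconnected.
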(fn `FireProjectile`
  (params (TargetActor :type "Actor Object Reference"))
  (bind _returnvalue (+ (`Actor.K2_GetActorLocation` (`self.GetOwner`)) (`self.MuzzleOffset`)))
  (`|SpawnActorFromClass` (`self.ProjectileClass`) (`KismetMathLibrary.MakeTransform` _returnvalue (`KismetMathLibrary.FindLookAtRotation` _returnvalue (`Actor.K2_GetActorLocation` TargetActor))) "Undefined" "MultiplyWithRoot" null null))