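; Player combat component that delivers melee-style attack damage for the top-down character.
; ExecuteAttack gathers actors overlapping the owning character's HitBox and reads each one's team through the BPI_TeamAgent interface.
; It applies base damage only to targets on a different team, preventing friendly fire, and credits the character and its controller as causer and instigator.
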(fn `Execute Attack`
  (bind _asbp_top_down_character (cast `/Game/Characters/Player/Blueprints/BP_TopDownCharacter` (`self.Owning Actor`)))
  (for _array_element (`PrimitiveComponent.GetOverlappingActors` (`/Game/Characters/Player/Blueprints/BP_TopDownCharacter.HitBox` _asbp_top_down_character) null)
    (bind _asbpi_team_agent (cast `/Game/GenericComponents/BPI_TeamAgent` _array_element))
    ; Friendly Fire Detection
    (bind _team (`/Game/GenericComponents/BPI_TeamAgent.get Team` _asbpi_team_agent))
    (bind _asbp_top_down_character_2 (cast `/Game/Characters/Player/Blueprints/BP_TopDownCharacter` (`self.Owning Actor`)))
    (bind _team_2 (`/Game/GenericComponents/BPI_TeamAgent.get Team` _asbp_top_down_character_2))
    (if (not (`|EnumEquality` _team _team_2))
      (`GameplayStatics.ApplyDamage` _array_element (`self.Base Damage`) (`Pawn.GetController` _asbp_top_down_character_2) _asbp_top_down_character_2))))