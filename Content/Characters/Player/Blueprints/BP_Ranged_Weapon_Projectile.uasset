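; Projectile actor for a ranged weapon that damages characters of an opposing team.
; It activates its projectile movement on BeginPlay and detects hits through a sphere overlap.
; Friendly fire is prevented by comparing the target's BPI_TeamAgent team with that of the instigating BP_TopDownCharacter.
; Only an opposing-team hit applies damage credited to the instigator and destroys the projectile; other overlaps are ignored.
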(event `self.ReceiveBeginPlay`
  (`ActorComponent.Activate` (`self.ProjectileMovement`) false))

(event `self.Sphere1.OnComponentBeginOverlap`
  (params (OverlappedComponent :type "PrimitiveComponent Object Reference") (OtherActor :type "Actor Object Reference") (OtherComp :type "PrimitiveComponent Object Reference") (OtherBodyIndex :type Integer) (bFromSweep :type Boolean) (SweepResult :type "HitResult Structure (by ref)"))
  (bind _asbpi_team_agent (cast `/Game/GenericComponents/BPI_TeamAgent` OtherActor))
  ; Friendly Fire Detection
  (bind _team (`/Game/GenericComponents/BPI_TeamAgent.get Team` _asbpi_team_agent))
  (bind _asbp_top_down_character (cast `/Game/Characters/Player/Blueprints/BP_TopDownCharacter` (`self.InstigatorActor`)))
  (bind _team_2 (`/Game/GenericComponents/BPI_TeamAgent.get Team` _asbp_top_down_character))
  (if (not (`|EnumEquality` _team _team_2))
    (`GameplayStatics.ApplyDamage` OtherActor (`self.Damage`) (`Pawn.GetController` _asbp_top_down_character) _asbp_top_down_character)
    (`self.K2_DestroyActor`)))

(fn `UserConstructionScript`)