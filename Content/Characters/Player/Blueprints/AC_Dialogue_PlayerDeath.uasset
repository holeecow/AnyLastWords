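; Player-death dialogue component in which Judas taunts Kairos and offers a choice of last words that grants a stat boost.
; The Dialogue override chains AddDialogue calls, advancing on each Pass Through state, with a key choice drawing one random line each for Attack, Speed and Health.
; After the farewell, it clears dialogue progress, adds the chosen flat stat increase through MyGameInstance and closes the conversation.
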(fn `Dialogue`
  (`parent.Dialogue`)
  (switch `int` (`self.DialogueTreeIndex`)
    (:`0`
      (bind _state (`self.AddDialogue` "Judas" "Kairos, you'll never be able to defeat me. Why do you try so hard?" (`|MakeArray` "Continue" :!type "Text")))
      (switch `/Game/GenericComponents/Dialogue/EDialogueState` _state
        (:`NewEnumerator0`
          (bind _state_2 (`self.AddDialogue` "Judas" "The outcome will never change to matter how many times you try." (`|MakeArray` "Continue" :!type "Text")))
          (switch `/Game/GenericComponents/Dialogue/EDialogueState` _state_2
            (:`NewEnumerator0`
              (bind _state_3 (`self.AddDialogue` "Judas" "So I ask you again..." (`|MakeArray` "Continue" :!type "Text")))
              (switch `/Game/GenericComponents/Dialogue/EDialogueState` _state_3
                (:`NewEnumerator0`
                  ; Player choices - 0 for attack, 1 for speed, 2 for health
                  (bind (_state_4 _optionindex) (`self.AddDialogue` "Judas" "Any last words?" (`|MakeArray` (`KismetArrayLibrary.Array_Random` (`|MakeArray` "(Attack) Mark my words, I'll be back stronger." "(Attack) I'll train harder and be back. Get ready Judas." "(Attack) Every drop of my blood spilled is an ounce of power returned." :!type "Text")) (`KismetArrayLibrary.Array_Random` (`|MakeArray` "(Speed) You won't even be able to catch me next time." "(Speed) Next time, you’ll be swinging at the wind." "(Speed) Strike all you like—I won't be there to receive it." :!type "Text")) (`KismetArrayLibrary.Array_Random` (`|MakeArray` "(Health) Your weapons have been feeling dull. Don't get complacent." "(Health) The pain has felt rather muted lately." "(Health) Your next blade will find my flesh a little harder to part." :!type "Text"))) null true))
                  (switch `/Game/GenericComponents/Dialogue/EDialogueState` _state_4
                    (:`NewEnumerator0`
                      (set `self.Choice` _optionindex)
                      (bind _state_5 (`self.AddDialogue` "Judas" "Better luck next time. Goodbye." (`|MakeArray` "Continue" :!type "Text")))
                      (switch `/Game/GenericComponents/Dialogue/EDialogueState` _state_5
                        (:`NewEnumerator0`
                          (`self.ClearDialogueProgress`)
                          (switch `int` (`self.Choice`)
                            (:`0`
                              ; Increase stats according to choice at end of conversation
                              (bind _asmy_game_instance (cast `/Game/GenericComponents/MyGameInstance` (`GameplayStatics.GetGameInstance`)))
                              (`/Game/GenericComponents/MyGameInstance.AddAttackAbsolute` _asmy_game_instance 10.0))
                            (:`1`
                              (bind _asmy_game_instance_2 (cast `/Game/GenericComponents/MyGameInstance` (`GameplayStatics.GetGameInstance`)))
                              (`/Game/GenericComponents/MyGameInstance.AddSpeedAbsolute` _asmy_game_instance_2 50.0))
                            (:`2`
                              (bind _asmy_game_instance_3 (cast `/Game/GenericComponents/MyGameInstance` (`GameplayStatics.GetGameInstance`)))
                              (`/Game/GenericComponents/MyGameInstance.AddHealthAbsolute` _asmy_game_instance_3 30.0)))
                          (`self.CloseConversation`))))))))))))))