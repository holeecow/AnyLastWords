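; Base dialogue component that opens a dialogue widget and runs branching conversations, notifying the owner when they close.
; Children presumably override the empty Dialogue function with AddDialogue calls, which replay from the start after each selection.
; A progress map returns saved choices for answered lines; the first unanswered one updates the widget, and removing entries allows backtracking.
; Optional audio plays each line's clip or a random default, async-loading soft references as needed.
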(event `self.ReceiveBeginPlay`
  (if (`self.UseAudio?`)
    (bind _returnvalue (`|AddComponentByClass` :`self` (`self.GetOwner`) :`Class` "/Script/Engine.AudioComponent"))
    (set `self.AudioComponent` _returnvalue)))

(event `LoadAndPlayDialogueAudioAsync`
  (params (SoundBase :type "SoundBase Soft Object Reference"))
  (bind _object (`|LoadAsset` SoundBase)
    (:`Completed`
      (bind _assound_base (cast `SoundBase` _object))
      (`AudioComponent.SetSound` (`self.AudioComponent`) _assound_base)
      (`AudioComponent.Play` (`self.AudioComponent`) 0.0))))

(fn `AddDialogue`
  (params (SpeakerName :type Text) (DialogueText :type Text) (OptionsText :type "Array of Text") (DialogueAudio :type "SoundBase Soft Object Reference") (isKeyDialogue :type Boolean) (CutsceneImage :type "Texture2D Object Reference"))
  (returns (State :type "/Game/GenericComponents/Dialogue/EDialogueState Enum") (OptionIndex :type Integer))
  (bind (_value _returnvalue) (`BlueprintMapLibrary.Map_Find` (`self.DialogueProgress`) (`self.DialogueIndex`)))
  ; Increment current Dialogue Index, then check if it has already been shown before
  (`/Engine/EditorBlueprintResources/StandardMacros.IncrementInt` (`self.DialogueIndex`)
    (:`  `
      (if _returnvalue
        ; If yes, just return
        (return "NewEnumerator0" _value)
        (else
          ; Else, update the text in the UI and play given audio file
          (`/Game/UI/Dialogue/UI_Dialogue.UpdateDialogueText` (`self.DialogueWidget`) (`self.DialogueIndex`) SpeakerName DialogueText OptionsText isKeyDialogue CutsceneImage)
          (`self.PlayDialogueAudio` DialogueAudio)
          (return "NewEnumerator1" 0))))))

(fn `ClearDialogueProgress`
  (`BlueprintMapLibrary.Map_Clear` (`self.DialogueProgress`)))

(fn `CloseConversation`
  (`Widget.RemoveFromParent` (`self.DialogueWidget`))
  (bind _audiocomponent (`self.AudioComponent`)
    (:`then`
      (`AudioComponent.Stop` _audiocomponent))
    (:`else`
      _))
  (message `/Game/GenericComponents/BPI_Interactable.ConversationClosed` (`self.GetOwner`)))

(fn `Dialogue`)

(fn `OpenConversation`
  (bind _returnvalue (`|CreateWidget` "/Game/UI/Dialogue/UI_Dialogue.UI_Dialogue_C" null self))
  (bind _output_get (set `self.DialogueWidget` _returnvalue))
  (`UserWidget.AddToViewport` _output_get 0)
  (`self.ProgressDialogue`))

(fn `PlayDialogueAudio`
  (params (Audio :type "SoundBase Soft Object Reference (by ref)"))
  (bind _output (`|ConvertAsset` (`self.ActiveAudio`)))
  (if (`self.UseAudio?`)
    ; Check if audio file is given
    (if (`KismetSystemLibrary.IsValidSoftObjectReference` Audio)
      ; If audio file given, set that as active audio
      (set `self.ActiveAudio` Audio)
      ; If soft ref resolves to concrete ref, set the audio component sound and play
      (`/Engine/EditorBlueprintResources/StandardMacros.IsValid` _output :!label _label
        (:`Is Valid`
          (`AudioComponent.SetSound` (`self.AudioComponent`) _output)
          (`AudioComponent.Play` (`self.AudioComponent`) 0.0))
        (:`Is Not Valid`
          ; If not, then load it async, and set and play
          (`self.LoadAndPlayDialogueAudioAsync` (`self.ActiveAudio`))))
      (else
        ; Audio file not given, pick one from default audio set
        (if (`BlueprintSetLibrary.Set_IsNotEmpty` (`self.DefaultAudio`))
          (bind _result (`BlueprintSetLibrary.Set_ToArray` (`self.DefaultAudio`)))
          (set `self.ActiveAudio` (`KismetArrayLibrary.Array_Random` _result))
          (goto _label))))))

(fn `ProgressDialogue`
  (set `self.DialogueIndex` -1)
  (`self.Dialogue`))

(fn `RemoveDialogueProgress`
  (params (ProgressSteps :type Integer))
  ; To backtrack within a branch
  (for _index (range (+ ProgressSteps 1))
    (`BlueprintMapLibrary.Map_Remove` (`self.DialogueProgress`) (- (`self.DialogueIndex`) _index))))

(fn `SetDialogueTreeIndex`
  (params (DialogueTreeIndex :type Integer))
  (set `self.DialogueTreeIndex` DialogueTreeIndex)
  (`self.ClearDialogueProgress`))

(fn `UpdateSelectedOption`
  (params (ProgressIndex :type "Integer (by ref)") (OptionIndex :type "Integer (by ref)"))
  ; Update dialogue progress map with the dialogue index and corresponding selected option, then progress dialogue
  (`BlueprintMapLibrary.Map_Add` (`self.DialogueProgress`) ProgressIndex OptionIndex)
  (`self.ProgressDialogue`))