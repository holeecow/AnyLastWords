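; Test dialogue component that scripts a branching friendship conversation with Alice and Boxie by overriding the parent's Dialogue function.
; DialogueTreeIndex selects one of three trees: first meeting, accepted friendship, or refused friendship with an audio ding and a second chance.
; Each AddDialogue call advances on its Pass Through state and branches on the chosen option.
; Endings switch the tree index or remove or clear dialogue progress before closing the conversation.
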(fn `Dialogue`
  (`parent.Dialogue`)
  (switch `int` (`self.DialogueTreeIndex`)
    (:`0`
      (bind _state (`self.AddDialogue` "Alice" "Hi! My name is Alice." (`|MakeArray` "Continue" :!type "Text")))
      (switch `/Game/GenericComponents/Dialogue/EDialogueState` _state
        (:`NewEnumerator0`
          (bind (_state_2 _optionindex) (`self.AddDialogue` "Alice" "Would you like to be my friend?" (`|MakeArray` "Of course!" "Not really..." :!type "Text")))
          (switch `/Game/GenericComponents/Dialogue/EDialogueState` _state_2
            (:`NewEnumerator0`
              (switch `int` _optionindex
                (:`0`
                  (bind _state_3 (`self.AddDialogue` "Alice" "Thank you! Let's be friends :)" (`|MakeArray` "Continue" :!type "Text")))
                  (switch `/Game/GenericComponents/Dialogue/EDialogueState` _state_3
                    (:`NewEnumerator0`
                      (`self.SetDialogueTreeIndex` 1)
                      (`self.CloseConversation`))))
                (:`1`
                  (bind _state_4 (`self.AddDialogue` "Alice" "Now, I'm sad :(" (`|MakeArray` "Continue" :!type "Text")))
                  (switch `/Game/GenericComponents/Dialogue/EDialogueState` _state_4
                    (:`NewEnumerator0`
                      (`self.SetDialogueTreeIndex` 2)
                      (`self.CloseConversation`))))))))))
    (:`1`
      (bind _state_5 (`self.AddDialogue` "Alice" "Hello again!" (`|MakeArray` "Continue" :!type "Text")))
      (switch `/Game/GenericComponents/Dialogue/EDialogueState` _state_5
        (:`NewEnumerator0`
          (bind _state_6 (`self.AddDialogue` "Alice" "Thanks for agreeing to be my friend. I'm happy!" (`|MakeArray` "Continue" :!type "Text")))
          (switch `/Game/GenericComponents/Dialogue/EDialogueState` _state_6
            (:`NewEnumerator0`
              (`self.RemoveDialogueProgress` 0)
              (`self.CloseConversation`))))))
    (:`2`
      (bind _state_7 (`self.AddDialogue` "Boxie" "Hello" (`|MakeArray` "Continue" :!type "Text") "/Game/Audio/SFX/SW_Ding.SW_Ding"))
      (switch `/Game/GenericComponents/Dialogue/EDialogueState` _state_7
        (:`NewEnumerator0`
          (bind (_state_8 _optionindex_2) (`self.AddDialogue` "Alice" "Would you like to be my friend now?" (`|MakeArray` "Yes" "Nah" :!type "Text")))
          (switch `/Game/GenericComponents/Dialogue/EDialogueState` _state_8
            (:`NewEnumerator0`
              (switch `int` _optionindex_2
                (:`0`
                  (bind _state_9 (`self.AddDialogue` "Boxie" "Great! Let's be friends." (`|MakeArray` "Continue" :!type "Text")))
                  (switch `/Game/GenericComponents/Dialogue/EDialogueState` _state_9
                    (:`NewEnumerator0`
                      (`self.SetDialogueTreeIndex` 1)
                      (`self.CloseConversation`))))
                (:`1`
                  (bind _state_10 (`self.AddDialogue` "Boxie" "Alright..." (`|MakeArray` "Continue" :!type "Text")))
                  (switch `/Game/GenericComponents/Dialogue/EDialogueState` _state_10
                    (:`NewEnumerator0`
                      (`self.ClearDialogueProgress`)
                      (`self.CloseConversation`))))))))))))