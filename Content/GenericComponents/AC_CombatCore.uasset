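; AC_CombatCore is a generic combat component that gates attacks by its owning Character on target validity, range and cooldown.
; TryAttack checks those conditions, stores the target as CurrentTarget, calls ExecuteAttack, starts the cooldown and returns whether it attacked.
; ExecuteAttack is empty here, so no attack behavior is defined at this level.
; The cooldown clears CanAttack and restores it through a timer set by function name.
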(event `self.ReceiveBeginPlay`
  (bind _ascharacter (cast `Character` (`self.GetOwner`)))
  (set `self.Owning Actor` _ascharacter))

(fn `Check Can Attack`
  (params (`Target Actor` :type "Actor Object Reference"))
  (returns (`can Attack` :type Boolean))
  (bind _owning_actor (`self.Owning Actor`))
  (return (and (`self.canAttack`) (`KismetSystemLibrary.IsValid` `Target Actor`) (`KismetSystemLibrary.IsValid` _owning_actor) (<= (`KismetMathLibrary.Vector_Distance` (`Actor.K2_GetActorLocation` _owning_actor) (`Actor.K2_GetActorLocation` `Target Actor`)) (`self.Attack Range`)))))

(fn `Execute Attack`)

(fn `Reset Cooldown`
  (set `self.canAttack` true))

(fn `Start Cooldown`
  (set `self.canAttack` false)
  (`KismetSystemLibrary.K2_SetTimer` null "Reset Cooldown" (`self.Attack Cooldown`)))

(fn `Try Attack`
  (params (`Target Actor` :type "Actor Object Reference"))
  (returns (isSucessful :type Boolean))
  (bind _can_attack (`self.Check Can Attack` `Target Actor`))
  (if _can_attack
    (set `self.Current Target` `Target Actor`)
    (`self.Execute Attack`)
    (`self.Start Cooldown`)
    (return true)
    (else
      (return false))))