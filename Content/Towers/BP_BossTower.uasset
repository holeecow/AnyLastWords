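; Boss tower enemy that fires radial projectile bursts at opposing-team actors in range and spawns minions when destroyed.
; A looping timer picks a target from the range sphere list, then timers drive an idle, charge, burst and cooldown state machine.
; Tick eases the turret toward its target during charge and burst, rotating the evenly spaced effect and projectile ring.
; Damage updates a health widget and spawns popups; death adds kill count and explodes.
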(event `self.ReceiveBeginPlay`
  (`KismetSystemLibrary.K2_SetTimerDelegate` (delegate `TryFire`) 1.0 true)
  (set `self.Health` (`self.MaxHealth`))
  (bind _returnvalue (`|CreateWidget` "/Game/Characters/Minion/WBP_MinionHealth.WBP_MinionHealth_C" null (`self.Health`) (`self.MaxHealth`) (`self.Name`) (`self.HealthColor`) 170.0))
  (set `self.HPWidget` _returnvalue)
  (`WidgetComponent.SetWidget` (`self.HealthUI`) _returnvalue)
  (`/Game/Characters/Minion/WBP_MinionHealth.UpdateHPBar` _returnvalue)
  (`/Game/Characters/Minion/WBP_MinionHealth.UpdateStyling` _returnvalue))

(event `TryFire`
  (if (and (> (`KismetArrayLibrary.Array_Length` (`self.ThisTowersTargetsInRange`)) 0) (`|EnumEquality` (`self.TowerState`) "NewEnumerator0"))
    (bind _chosen (`self.chooseTarget`))
    (`/Engine/EditorBlueprintResources/StandardMacros.IsValid` _chosen
      (:`Is Valid`
        (set `self.currtargeT` _chosen)
        (`self.start chrage`)))))

(event `start chrage`
  (bind _rotatecentre (`self.rotateCentre`))
  (bind (_returnvalue_roll _returnvalue_pitch _returnvalue_yaw) (`KismetMathLibrary.BreakRotator` (`SceneComponent.K2_GetComponentRotation` _rotatecentre)))
  (set `self.TowerState` "NewEnumerator1")
  (for _index (range (`self.Shots per burst`))
    (bind _returnvalue (+ (* _index (/ 360 (`self.Shots per burst`))) _returnvalue_yaw))
    (bind _returnvalue_2 (`NiagaraFunctionLibrary.SpawnSystemAtLocation` (`self.Charge effect system`) (+ (`SceneComponent.K2_GetComponentLocation` _rotatecentre) (* (`KismetMathLibrary.MakeVector` (`KismetMathLibrary.DegCos` _returnvalue) (`KismetMathLibrary.DegSin` _returnvalue)) 100.0)) (`KismetMathLibrary.MakeRotator` _returnvalue_roll _returnvalue_pitch _returnvalue) (1.0 1.0 1.0) false)))
  (`KismetSystemLibrary.K2_SetTimerDelegate` (delegate `FinishChrageup`) 4.0))

(event `FinishChrageup`
  (`/Engine/EditorBlueprintResources/StandardMacros.IsValid` (`self.currtargeT`)
    (:`Is Valid`
      (`ActorComponent.Deactivate` (stale `start chrage` _returnvalue_2))
      (`self.StartBurst`))
    (:`Is Not Valid`
      (set `self.TowerState` "NewEnumerator0"))))

(event `StartBurst`
  (set `self.TowerState` "NewEnumerator2")
  (set `self.BurstsRemaining` (`self.Bursts`))
  (`self.FireOneShot`))

(event `FireOneShot`
  (bind _rotatecentre (`self.rotateCentre`))
  (bind (_returnvalue_roll _returnvalue_pitch _returnvalue_yaw) (`KismetMathLibrary.BreakRotator` (`SceneComponent.K2_GetComponentRotation` _rotatecentre)))
  (for _index (range (`self.Shots per burst`))
    (bind _returnvalue (+ (* _index (/ 360 (`self.Shots per burst`))) _returnvalue_yaw))
    (`|SpawnActorFromClass` (`self.ProjectileClass`) (`KismetMathLibrary.MakeTransform` (+ (`SceneComponent.K2_GetComponentLocation` _rotatecentre) (* (`KismetMathLibrary.MakeVector` (`KismetMathLibrary.DegCos` _returnvalue) (`KismetMathLibrary.DegSin` _returnvalue)) 100.0)) (`KismetMathLibrary.MakeRotator` _returnvalue_roll _returnvalue_pitch _returnvalue)) "Undefined" "MultiplyWithRoot" null self null))
  (`KismetSystemLibrary.PrintString` "firing" true true (struct :`R` 1.0 :`G` 0.026135 :`A` 1.0))
  (bind _output_get (set `self.BurstsRemaining` (- (`self.BurstsRemaining`) 1)))
  (if (> _output_get 0)
    (`KismetSystemLibrary.K2_SetTimerDelegate` (delegate `FireOneShot`) (`self.BurstInterval`))
    (else
      (`self.StartCooldown`))))

(event `StartCooldown`
  (set `self.TowerState` "NewEnumerator3")
  (`MeshComponent.SetOverlayMaterial` (`self.tower`) "/Game/Towers/M_CooldownTele.M_CooldownTele")
  (`KismetSystemLibrary.K2_SetTimerDelegate` (delegate `FinishOOLDOWN`) 3.0))

(event `FinishOOLDOWN`
  (`MeshComponent.SetOverlayMaterial` (`self.tower`) null)
  (set `self.TowerState` "NewEnumerator0"))

(event `self.range Sphere.OnComponentBeginOverlap`
  (params (OverlappedComponent :type "PrimitiveComponent Object Reference") (OtherActor :type "Actor Object Reference") (OtherComp :type "PrimitiveComponent Object Reference") (OtherBodyIndex :type Integer) (bFromSweep :type Boolean) (SweepResult :type "HitResult Structure (by ref)"))
  ; Target Selection
  (bind _team (message `/Game/GenericComponents/BPI_TeamAgent.get Team` OtherActor))
  (if (`|EnumInequality` _team (`self.Team`))
    (`KismetArrayLibrary.Array_Append` (`self.ThisTowersTargetsInRange`) (`|MakeArray` OtherActor))))

(event `self.range Sphere.OnComponentEndOverlap`
  (params (OverlappedComponent :type "PrimitiveComponent Object Reference") (OtherActor :type "Actor Object Reference") (OtherComp :type "PrimitiveComponent Object Reference") (OtherBodyIndex :type Integer))
  ; Target Selection
  (`KismetArrayLibrary.Array_RemoveItem` (`self.ThisTowersTargetsInRange`) OtherActor))

(event `self.ReceiveAnyDamage`
  (params (Damage :type "Float (single-precision)") (DamageType :type "DamageType Object Reference") (InstigatedBy :type "Controller Object Reference") (DamageCauser :type "Actor Object Reference"))
  (bind _health (`self.Health`))
  ; taken from genric attackable
  (`|ExecutionSequence`
    (:`then_0`
      (set `self.Health` (- _health Damage))
      (bind _aswbp_minion_health (cast `/Game/Characters/Minion/WBP_MinionHealth` (`WidgetComponent.GetUserWidgetObject` (`self.HealthUI`))))
      (set `/Game/Characters/Minion/WBP_MinionHealth.CurrentHP` (`self.Health`) _aswbp_minion_health)
      (`/Game/Characters/Minion/WBP_MinionHealth.UpdateHPBar` _aswbp_minion_health)
      (if (<= _health 0.0)
        ;; might need to remove from minions in range
        (`self.HandleDeath`)))
    (:`then_1`
      (`|SpawnActorFromClass` "/Game/Characters/Minion/BP_DamagePopUp.BP_DamagePopUp_C" (`KismetMathLibrary.MakeTransform` (+ (`self.K2_GetActorLocation`) (0.0 0.0 160.0))) "Undefined" "MultiplyWithRoot" null (`KismetTextLibrary.Conv_DoubleToText` Damage "HalfToEven") (`self.HealthColor`) null))))

(event `self.ReceiveTick`
  (params (DeltaSeconds :type "Float (single-precision)"))
  (bind _rotatecentre (`self.rotateCentre`))
  (bind _currtarget (`self.currtargeT`))
  (bind _towerstate (`self.TowerState`))
  ; smooth turret tracking
  (`/Engine/EditorBlueprintResources/StandardMacros.IsValid` _currtarget
    (:`Is Valid`
      (if (or (`|EnumEquality` _towerstate "NewEnumerator1") (`|EnumEquality` _towerstate "NewEnumerator2"))
        (`SceneComponent.K2_SetWorldRotation` _rotatecentre (`KismetMathLibrary.RInterpTo` (`SceneComponent.K2_GetComponentRotation` _rotatecentre) (`KismetMathLibrary.FindLookAtRotation` (`SceneComponent.K2_GetComponentLocation` (`self.rotateCentre`)) (`self.K2_GetActorLocation` _currtarget)) DeltaSeconds 5.0) false false)))))

(event `/Game/GenericComponents/BPI_TeamAgent.ReleaseSlot`
  ; ReleaseSlot
  (if (> (`self.Slots`) 0)
    (set `self.Slots` (- (`self.Slots`) 1))))

(event `/Game/GenericComponents/BPI_Attackable.Attack`
  (params (Target :type "Actor Object Reference")))

(fn `get Team`
  (returns (Team :type "/Game/GenericComponents/ETeam Enum"))
  (return (`self.Team`)))

(fn `HandleDeath`
  (bind _returnvalue (`SceneComponent.K2_GetComponentLocation` (`self.DefaultSceneRoot`)))
  (bind _asmy_game_instance (cast `/Game/GenericComponents/MyGameInstance` (`GameplayStatics.GetGameInstance`)))
  (`/Game/GenericComponents/MyGameInstance.AddKillcount` _asmy_game_instance 10)
  (`NiagaraFunctionLibrary.SpawnSystemAtLocation` "/Game/Fab/MixedVFX/Particles/Explosions/NS_ExplosionGroundBig.NS_ExplosionGroundBig" _returnvalue)
  (`GameplayStatics.PlaySoundAtLocation` "/Game/Towers/freesound_community-medium-explosion-40472.freesound_community-medium-explosion-40472" _returnvalue (struct) 1.0 1.0 0.0 null null null null)
  (`self.spawn minion from tower` (`SceneComponent.K2_GetComponentToWorld` (`self.DefaultSceneRoot`)) (`self.NumMinionsToSpawn`))
  (`self.K2_DestroyActor`)
  (return))

(fn `SetSummonedVariant`
  (`parent.SetSummonedVariant`)
  (`KismetSystemLibrary.PrintString` "Hello" true true (struct :`R` 0.953527 :`G` 1.0 :`A` 1.0)))

(fn `UserConstructionScript`
  (`parent.UserConstructionScript`))