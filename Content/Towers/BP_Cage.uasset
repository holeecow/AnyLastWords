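; Destructible cage that holds a captive friendly minion and releases it when destroyed.
; BeginPlay randomly keeps the default minion type or switches to the ranged one with a matching mesh, then builds the health bar widget.
; Damage updates the bar and spawns a number popup; at zero health the cage explodes, calls the minion spawn and destroys itself.
; Attack-slot and target-score functions are stubs offering no slots and zero score.
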(event `self.ReceiveBeginPlay`
  (`|ExecutionSequence`
    (:`then_0`
      (if (== (`KismetMathLibrary.RandomIntegerInRange` 0 1) 0)
        (set `self.friendlyType` "/Game/Characters/Minion/Friendly/Ranged/BP_Friendly_Range.BP_Friendly_Range_C")
        (`SkeletalMeshComponent.SetSkeletalMeshAsset` (`self.Mushroom_SK`) "/Game/Characters/Minion/Friendly/Ranged/Swarm08_SK.Swarm08_SK")))
    (:`then_1`
      (set `self.Health` (`self.MaxHealth`))
      (bind _returnvalue (`|CreateWidget` "/Game/Characters/Minion/WBP_MinionHealth.WBP_MinionHealth_C" null (`self.Health`) (`self.MaxHealth`) (`self.Name`) (`self.HealthColor`) 170.0))
      (`WidgetComponent.SetWidget` (`self.HealthUI`) _returnvalue)
      (`/Game/Characters/Minion/WBP_MinionHealth.UpdateHPBar` _returnvalue)
      (`/Game/Characters/Minion/WBP_MinionHealth.UpdateStyling` _returnvalue))))

(event `self.ReceiveAnyDamage`
  (params (Damage :type "Float (single-precision)") (DamageType :type "DamageType Object Reference") (InstigatedBy :type "Controller Object Reference") (DamageCauser :type "Actor Object Reference"))
  (bind _health (`self.Health`))
  ; taken from genric attackable
  (`|ExecutionSequence`
    (:`then_0`
      (set `self.Health` (- _health Damage))
      (bind _aswbp_minion_health (cast `/Game/Characters/Minion/WBP_MinionHealth` (`WidgetComponent.GetUserWidgetObject` (`self.HealthUI`))))
      (set `/Game/Characters/Minion/WBP_MinionHealth.CurrentHP` (`self.Health`) _aswbp_minion_health)
      (`/Game/Characters/Minion/WBP_MinionHealth.UpdateHPBar` _aswbp_minion_health)
      (if (<= _health 0.0)
        (`self.HandleDeath`)))
    (:`then_1`
      (`|SpawnActorFromClass` "/Game/Characters/Minion/BP_DamagePopUp.BP_DamagePopUp_C" (`KismetMathLibrary.MakeTransform` (+ (`self.K2_GetActorLocation`) (0.0 0.0 160.0))) "Undefined" "MultiplyWithRoot" null (`KismetTextLibrary.Conv_DoubleToText` Damage "HalfToEven") (`self.HealthColor`) null))))

(event `/Game/GenericComponents/BPI_TeamAgent.ReleaseSlot`)

(event `/Game/GenericComponents/BPI_Attackable.Attack`
  (params (Target :type "Actor Object Reference")))

(fn `CalculateTargetScore`
  (params (AttackerLocation :type "Vector Structure"))
  (returns (TargetScore :type "Float (double-precision)"))
  (return 0.0))

(fn `ClaimSlot`
  (returns (canClaim :type Boolean))
  (return false))

(fn `get Team`
  (returns (Team :type "/Game/GenericComponents/ETeam Enum"))
  (return (`self.Team`)))

(fn `HandleDeath`
  (bind _returnvalue (`SceneComponent.K2_GetComponentLocation` (`self.DefaultSceneRoot`)))
  (`NiagaraFunctionLibrary.SpawnSystemAtLocation` "/Game/Fab/MixedVFX/Particles/Explosions/NS_ExplosionGroundBig.NS_ExplosionGroundBig" _returnvalue)
  (`GameplayStatics.PlaySoundAtLocation` "/Game/Towers/freesound_community-medium-explosion-40472.freesound_community-medium-explosion-40472" _returnvalue (struct) 1.0 1.0 0.0 null null null null)
  (`KismetSystemLibrary.PrintString` "Hello")
  (`self.spawn minion from cage` (`SceneComponent.K2_GetComponentToWorld` (`self.Mushroom_SK`)) (`self.friendlyType`))
  (`self.K2_DestroyActor`))

(fn `HasOpenSlot`
  (returns (canClaim :type Boolean))
  (return false))

(fn `UserConstructionScript`)