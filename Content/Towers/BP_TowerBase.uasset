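; Base tower that auto-attacks the nearest other-team actor inside its range sphere and can itself be damaged and destroyed.
; A looping timer starts a state cycle: charge-up with scaling effect while turning toward the target, timed projectile burst, then cooldown, which currently resets immediately.
; As an attackable, it shows HP text and exposes team, limited attacker slots and a target score from health, slot use and distance.
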(event `self.ReceiveBeginPlay`
  (`KismetSystemLibrary.K2_SetTimerDelegate` (delegate `Try Fire`) 3.0 true)
  (set `self.Health` (`self.MaxHealth`)))

(event `Try Fire`
  (if (and (> (`KismetArrayLibrary.Array_Length` (`self.ThisTowersTargetsInRange`)) 0) (`|EnumEquality` (`self.TowerState`) "NewEnumerator0"))
    (bind _chosen (`self.chooseTarget`))
    (`/Engine/EditorBlueprintResources/StandardMacros.IsValid` _chosen
      (:`Is Valid`
        (set `self.currtargeT` _chosen)
        (`self.Start Charge Up`)))))

(event `Start Charge Up`
  (set `self.TowerState` "NewEnumerator1")
  (bind _returnvalue (`NiagaraFunctionLibrary.SpawnSystemAttached` (`self.Charge effect system`) (`self.muzzle`) "None" (0.0 0.0 0.0) (struct) "SnapToTarget"))
  (bind (_direction _size) (`Timeline|Timeline` :!via `PlayFromStart`)
    (:`Update`
      (`SceneComponent.SetRelativeScale3D` _returnvalue (`KismetMathLibrary.Conv_DoubleToVector` _size)))
    (:`Finished`
      (`KismetSystemLibrary.K2_SetTimerDelegate` (delegate `Finish Charge up`) 2.0))))

(event `Finish Charge up`
  (`/Engine/EditorBlueprintResources/StandardMacros.IsValid` (`self.currtargeT`)
    (:`Is Valid`
      (`ActorComponent.Deactivate` (stale `Start Charge Up` _returnvalue))
      (`self.Start Burst`))
    (:`Is Not Valid`
      (set `self.TowerState` "NewEnumerator0"))))

(event `Start Burst`
  (set `self.TowerState` "NewEnumerator2")
  (set `self.shots remaining` (`self.Shots per burst`))
  (`self.FireOne Shot`))

(event `FireOne Shot`
  (bind _returnvalue (`|SpawnActorFromClass` (`self.ProjectileClass`) (`SceneComponent.K2_GetComponentToWorld` (`self.muzzle`)) "Undefined" "MultiplyWithRoot" null null))
  (set `/Game/Towers/BP_TowerProjectile_Base.OwningTower` self _returnvalue)
  (`KismetSystemLibrary.PrintString` "firing" true true (struct :`R` 1.0 :`G` 0.026135 :`A` 1.0))
  (bind _output_get (set `self.shots remaining` (- (`self.shots remaining`) 1)))
  (if (> _output_get 0)
    (`KismetSystemLibrary.K2_SetTimerDelegate` (delegate `FireOne Shot`) (`self.BurstInterval`))
    (else
      (`self.Start Cooldown`))))

(event `Start Cooldown`
  (set `self.TowerState` "NewEnumerator3")
  (`KismetSystemLibrary.K2_SetTimerDelegate` :`Time` 0.5)
  (`self.Finish Cooldown`))

(event `Finish Cooldown`
  (set `self.TowerState` "NewEnumerator0"))

(event `self.range Sphere.OnComponentBeginOverlap`
  (params (OverlappedComponent :type "PrimitiveComponent Object Reference") (OtherActor :type "Actor Object Reference") (OtherComp :type "PrimitiveComponent Object Reference") (OtherBodyIndex :type Integer) (bFromSweep :type Boolean) (SweepResult :type "HitResult Structure (by ref)"))
  ; detection and tracking of good minions
  (bind _team (message `/Game/GenericComponents/BPI_TeamAgent.get Team` OtherActor))
  (if (`|EnumInequality` _team (`self.Team`))
    (`KismetArrayLibrary.Array_Append` (`self.ThisTowersTargetsInRange`) (`|MakeArray` OtherActor))))

(event `self.range Sphere.OnComponentEndOverlap`
  (params (OverlappedComponent :type "PrimitiveComponent Object Reference") (OtherActor :type "Actor Object Reference") (OtherComp :type "PrimitiveComponent Object Reference") (OtherBodyIndex :type Integer))
  ; detection and tracking of good minions
  (`KismetArrayLibrary.Array_RemoveItem` (`self.ThisTowersTargetsInRange`) OtherActor))

(event `self.ReceiveTick`
  (params (DeltaSeconds :type "Float (single-precision)"))
  (bind _rotatecentre (`self.rotateCentre`))
  ; taken from genric attackable
  (`TextRenderComponent.K2_SetText` (`self.HealthTextRender`) (`|GenericToText` (`KismetStringLibrary.Concat_StrStr` "HP: " (`KismetStringLibrary.Conv_DoubleToString` (`self.Health`)))))
  (if (`|EnumEquality` (`self.TowerState`) "NewEnumerator1")
    (`SceneComponent.K2_SetWorldRotation` _rotatecentre (`KismetMathLibrary.RInterpTo` (`SceneComponent.K2_GetComponentRotation` _rotatecentre) (`KismetMathLibrary.FindLookAtRotation` (`SceneComponent.K2_GetComponentLocation` (`self.rotateCentre`)) (`self.K2_GetActorLocation` (`self.currtargeT`))) DeltaSeconds 5.0) false false)))

(event `self.ReceiveAnyDamage`
  (params (Damage :type "Float (single-precision)") (DamageType :type "DamageType Object Reference") (InstigatedBy :type "Controller Object Reference") (DamageCauser :type "Actor Object Reference"))
  (bind _health (`self.Health`))
  ; taken from genric attackable
  (set `self.Health` (- _health Damage))
  (if (<= _health 0.0)
    ;; might need to remove from minions in range
    (`self.K2_DestroyActor`)))

(event `/Game/GenericComponents/BPI_Attackable.Attack`
  (params (Targett :type "Actor Object Reference")))

(event `/Game/GenericComponents/BPI_TeamAgent.ReleaseSlot`
  ; ReleaseSlot
  (if (> (`self.Slots`) 0)
    (set `self.Slots` (- (`self.Slots`) 1))))

(fn `CalculateTargetScore`
  (params (AttackerLocation :type "Vector Structure"))
  (returns (TargetScore :type "Float (double-precision)"))
  (locals (FinalScore :type "Float (double-precision)"))
  (bind _returnvalue (/ (`self.Slots`) (`self.MaxSlot`)))
  (bind _returnvalue_2 (/ (`self.Health`) (`self.MaxHealth`)))
  (`|ExecutionSequence`
    (:`then_0`
      ; Check Health
      (if (< _returnvalue_2 0.3)
        (set `local.FinalScore` (+ (`local.FinalScore`) 50.0))
        (elif (< _returnvalue_2 0.7)
          (set `local.FinalScore` (+ (`local.FinalScore`) 30.0))
          (else
            (set `local.FinalScore` (+ (`local.FinalScore`) 10.0))))))
    (:`then_1`
      ; Check Slot
      (if (< _returnvalue 0.2)
        (set `local.FinalScore` (+ (`local.FinalScore`) 50.0))
        (elif (> _returnvalue 1.0)
          (set `local.FinalScore` (+ (`local.FinalScore`) 0.0))
          (else
            (set `local.FinalScore` (+ (`local.FinalScore`) 20.0))))))
    (:`then_2`
      ; Check Distance
      (set `local.FinalScore` (- (`local.FinalScore`) (/ (`KismetMathLibrary.Vector_Distance` AttackerLocation (`self.K2_GetActorLocation`)) 100.0))))
    (:`then_3`
      ; Output
      (return (`local.FinalScore`)))))

(fn `chooseTarget`
  (returns (chosen :type "Actor Object Reference"))
  (return (`.ReturnValue` (`GameplayStatics.FindNearestActor` (`self.K2_GetActorLocation`) (`self.ThisTowersTargetsInRange`)))))

(fn `ClaimSlot`
  (returns (canClaim :type Boolean))
  (bind _canclaim (`self.HasOpenSlot`))
  (if _canclaim
    (set `self.Slots` (+ (`self.Slots`) 1))
    (return true)
    (else
      (return false))))

(fn `ExecuteFire`
  (bind _rotatecentre (`self.rotateCentre`))
  (`SceneComponent.K2_SetWorldRotation` _rotatecentre (`KismetMathLibrary.RInterpTo` (`SceneComponent.K2_GetComponentRotation` _rotatecentre) (`KismetMathLibrary.FindLookAtRotation` (`SceneComponent.K2_GetComponentLocation` (`self.rotateCentre`)) (`self.K2_GetActorLocation` (`self.currtargeT`))) 0.01 50.0) false false)
  (bind _returnvalue (`|SpawnActorFromClass` (`self.ProjectileClass`) (`SceneComponent.K2_GetComponentToWorld` (`self.muzzle`)) "Undefined" "MultiplyWithRoot" null null))
  (set `/Game/Towers/BP_TowerProjectile_Base.OwningTower` self _returnvalue)
  (`KismetSystemLibrary.PrintString` "firing" true true (struct :`R` 1.0 :`G` 0.026135 :`A` 1.0)))

(fn `get Team`
  (returns (Team :type "/Game/GenericComponents/ETeam Enum"))
  (return (`self.Team`)))

(fn `HasOpenSlot`
  (returns (canClaim :type Boolean))
  (if (< (`self.Slots`) (`self.MaxSlot`))
    (return true)
    (else
      (return false))))

(fn `UserConstructionScript`)