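; BP_Shuriken is a tower-related shuriken Blueprint, likely a projectile, that inherits its behavior from a parent class.
; On BeginPlay it randomly sets CurveParam to a positive or negative value of equal magnitude, then calls the parent BeginPlay.
; Tick and the construction script only forward to the parent, and the overlap event is disabled, so how CurveParam is used lies outside this graph.
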(event `self.ReceiveBeginPlay`
  (if (`KismetMathLibrary.RandomBool`)
    (set `self.CurveParam` 120.0)
    (else
      (set `self.CurveParam` -120.0)))
  (`parent.ReceiveBeginPlay`))

(event `self.ReceiveTick`
  (params (DeltaSeconds :type "Float (single-precision)"))
  (`parent.ReceiveTick` DeltaSeconds))

(fn `UserConstructionScript`
  (`parent.UserConstructionScript`))