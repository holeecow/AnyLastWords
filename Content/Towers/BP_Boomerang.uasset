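; Boomerang projectile for a tower that flies out, then homes back to the tower that fired it.
; Two seconds after spawning, it sets the tower's rotation centre as the projectile movement's homing target.
; Its sphere overlap deals extra damage to characters.
; While homing, touching the owning tower's "destroybox" component spawns an attached particle effect and destroys the boomerang.
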(event `self.ReceiveBeginPlay`
  (`KismetSystemLibrary.Delay` 2.0)
  (`self.set homing`)
  (set `self.isHoming` true))

(event `self.Sphere.OnComponentBeginOverlap`
  (params (OverlappedComponent :type "PrimitiveComponent Object Reference") (OtherActor :type "Actor Object Reference") (OtherComp :type "PrimitiveComponent Object Reference") (OtherBodyIndex :type Integer) (bFromSweep :type Boolean) (SweepResult :type "HitResult Structure (by ref)"))
  (`/Engine/EditorBlueprintResources/StandardMacros.IsValid` OtherActor
    (:`Is Valid`
      (cast `Character` OtherActor
        (:`then`
          (`GameplayStatics.ApplyDamage` OtherActor (`self.ExtraDamage`) null (`self.OwningTower`)))
        (:`CastFailed`
          (if (and (`ActorComponent.ComponentHasTag` OtherComp "destroybox") (== OtherActor (`self.OwningTower`)) (`self.isHoming`))
            (`GameplayStatics.SpawnEmitterAttached` "/Engine/Tutorial/SubEditors/TutorialAssets/TutorialParticleSystem.TutorialParticleSystem")
            (`self.K2_DestroyActor`)))))))

(event `self.ReceiveActorBeginOverlap`
  (params (OtherActor :type "Actor Object Reference"))
  (`parent.ReceiveActorBeginOverlap` OtherActor))

(fn `set homing`
  (bind _projectilemovement (`self.ProjectileMovement`))
  (bind _owningtower (`self.OwningTower`))
  (`/Engine/EditorBlueprintResources/StandardMacros.IsValid` _owningtower
    (:`Is Valid`
      (set `ProjectileMovementComponent.bIsHomingProjectile` true _projectilemovement)
      (set `ProjectileMovementComponent.HomingTargetComponent` (`/Game/Towers/BP_TowerBase.rotateCentre` _owningtower) _projectilemovement))))

(fn `UserConstructionScript`
  (`parent.UserConstructionScript`))