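; Dialogue component for the first revive scene, where the player wakes outside Towervania and vows revenge on Judas.
; It overrides Dialogue to pause the game, disable player input and play a linear chain of single-option AddDialogue steps, each advancing on Pass Through.
; The last step calls CloseConversation, which runs the parent logic, then unpauses and restores input.
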(fn `CloseConversation`
  (`parent.CloseConversation`)
  (`GameplayStatics.SetGamePaused` false)
  (`Actor.EnableInput` (`GameplayStatics.GetPlayerController` 0) null))

(fn `Dialogue`
  (`parent.Dialogue`)
  (`GameplayStatics.SetGamePaused` true)
  (`Actor.DisableInput` (`GameplayStatics.GetPlayerController` 0) null)
  (bind _state (`self.AddDialogue` "" "You wake up in a wide open field..." (`|MakeArray` "..." :!type "Text")))
  (switch `/Game/GenericComponents/Dialogue/EDialogueState` _state
    (:`NewEnumerator0`
      (bind _state_2 (`self.AddDialogue` "" "" (`|MakeArray` "HUH... where am I? I thought Judas finished me off." :!type "Text")))
      (switch `/Game/GenericComponents/Dialogue/EDialogueState` _state_2
        (:`NewEnumerator0`
          (bind _state_3 (`self.AddDialogue` "" "" (`|MakeArray` "This is... the outskirts of Towervania..." :!type "Text")))
          (switch `/Game/GenericComponents/Dialogue/EDialogueState` _state_3
            (:`NewEnumerator0`
              (bind _state_4 (`self.AddDialogue` "" "" (`|MakeArray` "I don't know how I'm alive but..." :!type "Text")))
              (switch `/Game/GenericComponents/Dialogue/EDialogueState` _state_4
                (:`NewEnumerator0`
                  (bind _state_5 (`self.AddDialogue` "" "" (`|MakeArray` "Judas will pay." :!type "Text")))
                  (switch `/Game/GenericComponents/Dialogue/EDialogueState` _state_5
                    (:`NewEnumerator0`
                      (`self.CloseConversation`))))))))))))