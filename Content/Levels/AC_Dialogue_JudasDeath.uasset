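; Dialogue component for the death of Judas, playing his final exchange with Kairos and the narrated ending of the revenge story in Towervania.
; The Dialogue override calls its parent, then chains AddDialogue calls through their Pass Through state, each offering a single response, so the conversation is strictly linear.
; The closing narration lines omit a speaker name, and the last one calls CloseConversation, which only forwards to the parent.
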(fn `CloseConversation`
  (`parent.CloseConversation`))

(fn `Dialogue`
  (`parent.Dialogue`)
  (bind _state (`self.AddDialogue` "Judas" "How? This is impossible. I struck you down. I watched the life leave your eyes, over and over again!" (`|MakeArray` "Continue" :!type "Text")))
  (switch `/Game/GenericComponents/Dialogue/EDialogueState` _state
    (:`NewEnumerator0`
      (bind _state_2 (`self.AddDialogue` "Judas" "I was stronger, better than you!" (`|MakeArray` "You were, but every defeat only taught me how to break you eventually." :!type "Text")))
      (switch `/Game/GenericComponents/Dialogue/EDialogueState` _state_2
        (:`NewEnumerator0`
          (bind _state_3 (`self.AddDialogue` "Judas" "Wait, Kairos, think about this! The kingdom still needs the both of us. With my brains and your power, we could rule over Towervania and make it prosper!" (`|MakeArray` "..." :!type "Text")))
          (switch `/Game/GenericComponents/Dialogue/EDialogueState` _state_3
            (:`NewEnumerator0`
              (bind _state_4 (`self.AddDialogue` "Judas" "Fine, kill me then. But know in your heart that I was always the one meant to lead Towervania. You are just a wrathful monster that slays everything in your way." (`|MakeArray` "You’re right, and now, you’re the one in my way." :!type "Text")))
              (switch `/Game/GenericComponents/Dialogue/EDialogueState` _state_4
                (:`NewEnumerator0`
                  (bind _state_5 (`self.AddDialogue` "Judas" "YOU HAVEN’T SEEN THE LAST OF ME, KAIROS! FU-" (`|MakeArray` "Judas." :!type "Text")))
                  (switch `/Game/GenericComponents/Dialogue/EDialogueState` _state_5
                    (:`NewEnumerator0`
                      (bind _state_6 (`self.AddDialogue` "Judas" "WHAT??!?" (`|MakeArray` "Any last words?" :!type "Text")))
                      (switch `/Game/GenericComponents/Dialogue/EDialogueState` _state_6
                        (:`NewEnumerator0`
                          (bind _state_7 (`self.AddDialogue` "Judas" "Huh, so you did care for customs. Well, my last words are-" (`|MakeArray` "Finish him." :!type "Text")))
                          (switch `/Game/GenericComponents/Dialogue/EDialogueState` _state_7
                            (:`NewEnumerator0`
                              (bind _state_8 (`self.AddDialogue` "" "You finish him off. And when you do, you feel the cycle break. The journey of your revenge has finally come to an end." (`|MakeArray` "Continue" :!type "Text")))
                              (switch `/Game/GenericComponents/Dialogue/EDialogueState` _state_8
                                (:`NewEnumerator0`
                                  (bind _state_9 (`self.AddDialogue` "" "And with it, begins a new story, one where you rebuild the kingdom of Towervania with those still loyal to you, and ensure peace for all." (`|MakeArray` "Continue" :!type "Text")))
                                  (switch `/Game/GenericComponents/Dialogue/EDialogueState` _state_9
                                    (:`NewEnumerator0`
                                      (`self.CloseConversation`))))))))))))))))))))