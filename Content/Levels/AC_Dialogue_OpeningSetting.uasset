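; Dialogue component that plays the opening story: Kairos, commander of Towervania's army, defeats the orc Gromak and is then betrayed by his aide Judas.
; The Dialogue override runs a linear chain of AddDialogue nodes, each with a single response option and advancing on its Pass Through state.
; The last line calls CloseConversation, whose override runs the parent logic and then opens the Lvl_TopDown level.
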(fn `CloseConversation`
  (`parent.CloseConversation`)
  (`GameplayStatics.OpenLevel` "Lvl_TopDown"))

(fn `Dialogue`
  (`parent.Dialogue`)
  (bind _state (`self.AddDialogue` "" "You are Kairos, the prince of the Kingdom of Towervania." (`|MakeArray` "Continue" :!type "Text")))
  (switch `/Game/GenericComponents/Dialogue/EDialogueState` _state
    (:`NewEnumerator0`
      (bind _state_2 (`self.AddDialogue` "" "At a young age, you took up arms to join the army, and fought to keep the Kingdom safe from the threat of monsters." (`|MakeArray` "Continue" :!type "Text")))
      (switch `/Game/GenericComponents/Dialogue/EDialogueState` _state_2
        (:`NewEnumerator0`
          (bind _state_3 (`self.AddDialogue` "" "Your skills grew as you aged, and you eventually become the commander of Towervania's army." (`|MakeArray` "Continue" :!type "Text")))
          (switch `/Game/GenericComponents/Dialogue/EDialogueState` _state_3
            (:`NewEnumerator0`
              (bind _state_4 (`self.AddDialogue` "" "In a particularly gruesome battle, you were wounded badly, but you managed to best the Orcian tribe leader, Gromak." (`|MakeArray` "Continue" :!type "Text")))
              (switch `/Game/GenericComponents/Dialogue/EDialogueState` _state_4
                (:`NewEnumerator0`
                  (bind _state_5 (`self.AddDialogue` "Gromak" "That was a true battle indeed. I'm glad that it was you who bested me..." (`|MakeArray` "It was a good battle. Goodbye." :!type "Text")))
                  (switch `/Game/GenericComponents/Dialogue/EDialogueState` _state_5
                    (:`NewEnumerator0`
                      (bind _state_6 (`self.AddDialogue` "Gromak" "Wait wait... You aren't gonna ask me for my last words? I thought that was customa-" (`|MakeArray` "Continue" :!type "Text")))
                      (switch `/Game/GenericComponents/Dialogue/EDialogueState` _state_6
                        (:`NewEnumerator0`
                          (bind _state_7 (`self.AddDialogue` "" "You finish him off. And when you do, you felt something strange happen, but you ignore it. You have to get help and recover right now." (`|MakeArray` "Continue" :!type "Text")))
                          (switch `/Game/GenericComponents/Dialogue/EDialogueState` _state_7
                            (:`NewEnumerator0`
                              (bind _state_8 (`self.AddDialogue` "" "On the way back to the kingdom, you found Judas, one of your most trusted aides." (`|MakeArray` "Judas! I'm so glad to see you. I managed to vanquish Gromak, but I'm not doing too good myself. Could you help me back into the kingdom?" :!type "Text")))
                              (switch `/Game/GenericComponents/Dialogue/EDialogueState` _state_8
                                (:`NewEnumerator0`
                                  (bind _state_9 (`self.AddDialogue` "Judas" "..." (`|MakeArray` "Judas?" :!type "Text")))
                                  (switch `/Game/GenericComponents/Dialogue/EDialogueState` _state_9
                                    (:`NewEnumerator0`
                                      (bind _state_10 (`self.AddDialogue` "Judas" "Pathetic. I never knew how you managed to become the army's commander." (`|MakeArray` "... What?" :!type "Text")))
                                      (switch `/Game/GenericComponents/Dialogue/EDialogueState` _state_10
                                        (:`NewEnumerator0`
                                          (bind _state_11 (`self.AddDialogue` "Judas" "You are weak, look at you. Fighting a lowly orc shouldn't put the commander of the army in such a state." (`|MakeArray` "..." :!type "Text")))
                                          (switch `/Game/GenericComponents/Dialogue/EDialogueState` _state_11
                                            (:`NewEnumerator0`
                                              (bind _state_12 (`self.AddDialogue` "Judas" "I've been waiting for a time like this. It's time for me to be the commander of Towervania's army, as it always should have been." (`|MakeArray` "..." :!type "Text")))
                                              (switch `/Game/GenericComponents/Dialogue/EDialogueState` _state_12
                                                (:`NewEnumerator0`
                                                  (bind _state_13 (`self.AddDialogue` "Judas" "I guess this is it Kairos. I would say that it's been fun working with you, but it was absolutely miserable. Well then..." (`|MakeArray` "Continue" :!type "Text")))
                                                  (switch `/Game/GenericComponents/Dialogue/EDialogueState` _state_13
                                                    (:`NewEnumerator0`
                                                      (bind _state_14 (`self.AddDialogue` "Judas" "Any last words?" (`|MakeArray` "This won't be the last you see of me." :!type "Text")))
                                                      (switch `/Game/GenericComponents/Dialogue/EDialogueState` _state_14
                                                        (:`NewEnumerator0`
                                                          (bind _state_15 (`self.AddDialogue` "Judas" "Sure, goodbye Kairos." (`|MakeArray` "Continue" :!type "Text")))
                                                          (switch `/Game/GenericComponents/Dialogue/EDialogueState` _state_15
                                                            (:`NewEnumerator0`
                                                              (`self.CloseConversation`))))))))))))))))))))))))))))))))