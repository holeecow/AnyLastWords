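; Dialogue component for the player's second revive, in which a monologue hints that doing more each time makes them return stronger.
; Overrides Dialogue to pause the game, disable player input and chain four single-line AddDialogue calls, each advancing on the Pass Through state.
; The last line calls the CloseConversation override, which unpauses the game and re-enables input.
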(fn `CloseConversation`
  (`parent.CloseConversation`)
  (`GameplayStatics.SetGamePaused` false)
  (`Actor.EnableInput` (`GameplayStatics.GetPlayerController` 0) null))

(fn `Dialogue`
  (`parent.Dialogue`)
  (`GameplayStatics.SetGamePaused` true)
  (`Actor.DisableInput` (`GameplayStatics.GetPlayerController` 0) null)
  (bind _state (`self.AddDialogue` "" "" (`|MakeArray` "I'm back here again." :!type "Text")))
  (switch `/Game/GenericComponents/Dialogue/EDialogueState` _state
    (:`NewEnumerator0`
      (bind _state_2 (`self.AddDialogue` "" "" (`|MakeArray` "And I feel... stronger somehow." :!type "Text")))
      (switch `/Game/GenericComponents/Dialogue/EDialogueState` _state_2
        (:`NewEnumerator0`
          (bind _state_3 (`self.AddDialogue` "" "" (`|MakeArray` "I have a feeling that the more I do each time, the stronger I get when I'm back." :!type "Text")))
          (switch `/Game/GenericComponents/Dialogue/EDialogueState` _state_3
            (:`NewEnumerator0`
              (bind _state_4 (`self.AddDialogue` "" "" (`|MakeArray` "Time to test out this theory." :!type "Text")))
              (switch `/Game/GenericComponents/Dialogue/EDialogueState` _state_4
                (:`NewEnumerator0`
                  (`self.CloseConversation`))))))))))