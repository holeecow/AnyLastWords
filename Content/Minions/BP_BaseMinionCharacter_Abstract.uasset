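; Abstract base character for minions, providing team, health and death handling for derived minion types.
; Health starts at MaxHealth, drops on AnyDamage with a debug print, and at zero or below sets IsDead and destroys the actor through HandleDeath.
; Tick refreshes a text render component with current HP as a test readout.
; Attack is an empty event, and GetTeam exposes the minion's team.
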(event `self.ReceiveBeginPlay`
  (set `self.Health` (`self.MaxHealth`)))

(event `/Game/GenericComponents/BPI_Attackable.Attack`)

(event `self.ReceiveTick`
  (params (DeltaSeconds :type "Float (single-precision)"))
  ; from test attackable fro dealing damage
  (`TextRenderComponent.K2_SetText` (`self.Health TextRender`) (`|GenericToText` (`KismetStringLibrary.Concat_StrStr` "HP: " (`KismetStringLibrary.Conv_DoubleToString` (`self.Health`))))))

(event `self.ReceiveAnyDamage`
  (params (Damage :type "Float (single-precision)") (DamageType :type "DamageType Object Reference") (InstigatedBy :type "Controller Object Reference") (DamageCauser :type "Actor Object Reference"))
  (bind _health (`self.Health`))
  ; Take Damage
  (set `self.Health` (- _health Damage))
  (`KismetSystemLibrary.PrintString` (`KismetStringLibrary.Concat_StrStr` "Ouch, I got hit! HP Left: " (`KismetStringLibrary.Conv_DoubleToString` (`self.Health`))))
  (if (<= _health 0.0)
    (set `self.isDead` true)
    (`self.Handle Death`)))

(fn `get Team`
  (returns (Team :type "/Game/GenericComponents/ETeam Enum"))
  (return (`self.Team`)))

(fn `Handle Death`
  (set `self.isDead` true)
  (`self.K2_DestroyActor`))

(fn `UserConstructionScript`)