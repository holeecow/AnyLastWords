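; BP_Friendly_Melee is a friendly melee minion Blueprint that reports a fixed team through GetTeam.
; Interaction is delegated to the ACFollowOnInteract component, which receives the interactor through HandleInteract.
; An UpdateOverlayMaterial event applies the supplied overlay material to the mesh.
; The Attack event is empty, BeginPlay, overlap and Tick are disabled stubs, and construction only calls the parent.
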(event `/Game/GenericComponents/BPI_Attackable.Attack`
  (params (Target :type "Actor Object Reference")))

(event `/Game/GenericComponents/BPI_Interactable.BeInteractedWith`
  (params (Interactor :type "Actor Object Reference"))
  (`/Game/Minions/AC_FollowOnInteract.Handle Interact` (`self.AC_FollowOnInteract`) Interactor))

(event `UpdateOverlayMaterial`
  (params (OverlayMaterial :type "MaterialInstance Object Reference"))
  (`MeshComponent.SetOverlayMaterial` (`self.Mesh`) OverlayMaterial))

(fn `get Team`
  (returns (Team :type "/Game/GenericComponents/ETeam Enum"))
  (return "NewEnumerator0"))

(fn `UserConstructionScript`
  (`parent.UserConstructionScript`))